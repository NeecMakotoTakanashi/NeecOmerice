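; BP_TItleLogo is a title logo actor that plays a flipbook-style animation on its Front mesh.
; BeginPlay creates a dynamic material instance from Front's first material slot.
; StartAnimation waits briefly, then steps through the ColorTextures and AlphaTextures arrays one frame per tick, setting the Color and Alpha texture parameters.
; The sequence runs to the end of ColorTextures and does not reset the counter.
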(event Custom|StartAnimation
  (bind _colortextures (Variables|Default|GetColorTextures))
  (bind _counter (Variables|Default|GetCounter))
  (bind _frontdynamicmi (Variables|Default|GetFrontDynamicMI))
  (Utilities|FlowControl|Delay 0.4)
  (if (< _counter (Utilities|Array|Length _colortextures)) :!label _label
    (Rendering|Material|SetTextureParameterValue _frontdynamicmi "Color" (Utilities|Array|Get(acopy) _colortextures _counter))
    (Rendering|Material|SetTextureParameterValue _frontdynamicmi "Alpha" (Utilities|Array|Get(acopy) (Variables|Default|GetAlphaTextures) _counter))
    (Math|Integer|IncrementInt (Variables|Default|GetCounter)
      (:%20%20
        (Utilities|FlowControl|DelayUntilNextTick)
        (goto _label)))))

(event EventBeginPlay
  (bind _returnvalue (Rendering|Material|CreateDynamicMaterialInstance (Variables|Default|GetFront) 0 (Rendering|Material|GetMaterial (Variables|Default|GetFront) 0) "None" :!class /Script/Engine.PrimitiveComponent))
  (Variables|Default|SetFrontDynamicMI _returnvalue))

(fn ConstructionScript)