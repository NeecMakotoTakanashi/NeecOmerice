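; BP_TItleLogo_Front plays a one-shot texture-sequence animation on the front layer of the title logo.
; BeginPlay creates a dynamic material instance from the Front component's first material.
; Each Tick sets that material's Color and Alpha parameters from paired texture arrays and advances a counter, so playback speed follows frame rate.
; Updates stop after the last color texture, leaving that frame displayed.
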(event EventBeginPlay
  (bind _returnvalue (Rendering|Material|CreateDynamicMaterialInstance (Variables|Default|GetFront) 0 (Rendering|Material|GetMaterial (Variables|Default|GetFront) 0) "None" :!class /Script/Engine.PrimitiveComponent))
  (Variables|Default|SetFrontDynamicMI _returnvalue))

(event EventTick
  (params (DeltaSeconds :type Float%20%28single-precision%29))
  (bind _colortextures (Variables|Default|GetColorTextures))
  (bind _counter (Variables|Default|GetCounter))
  (bind _frontdynamicmi (Variables|Default|GetFrontDynamicMI))
  (if (< _counter (Utilities|Array|Length _colortextures))
    (Rendering|Material|SetTextureParameterValue _frontdynamicmi "Color" (Utilities|Array|Get(acopy) _colortextures _counter))
    (Rendering|Material|SetTextureParameterValue _frontdynamicmi "Alpha" (Utilities|Array|Get(acopy) (Variables|Default|GetAlphaTextures) _counter))
    (Math|Integer|IncrementInt (Variables|Default|GetCounter))))

(fn ConstructionScript)