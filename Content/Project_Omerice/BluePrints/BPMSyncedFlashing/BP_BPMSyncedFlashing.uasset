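; BP_BPMSyncedFlashing is an actor whose static mesh flashes in time with a configurable BPM.
; The construction script creates a dynamic instance of M_BPMSyncedFlashing, and TurnOn and TurnOff set its EmissiveIntensity.
; Tick accumulates time and restarts the flash every beat, using a half-beat Delay to toggle, with DownBeat shifting the lit half to the offbeat.
; EnableFlashing and DisableFlashing control it, optionally starting on BeginPlay through AutoEnable.
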(event Custom|TurnOn
  (Rendering|Material|SetScalarParameterValue (Variables|Default|GetDynamicMaterial) "EmissiveIntensity" (Variables|Default|GetIntensityTurnOn) :!class /Script/Engine.MaterialInstanceDynamic))

(event Custom|TurnOff
  (Rendering|Material|SetScalarParameterValue (Variables|Default|GetDynamicMaterial) "EmissiveIntensity" (Variables|Default|GetIntensityTurnOff) :!class /Script/Engine.MaterialInstanceDynamic))

(event Custom|EnableFlashing
  (bind _bpm (Variables|Default|GetBPM))
  (bind _returnvalue (/ _bpm 60))
  (bind _returnvalue_2 (/ 1e+03 _returnvalue))
  (bind _returnvalue_3 (* 0.001 _returnvalue_2))
  (bind _returnvalue_4 (/ _returnvalue_3 2.0))
  ;[1 1 1] 点滅開始
  (Variables|Default|SetFlashing true)
  (Variables|Default|SetTime 0.0)
  ;;[1 1 1] DownBeat = Trueにすると裏拍のタイミングで光る
  (if (Variables|Default|GetDownBeat)
    (CallFunction|TurnOff)
    (Utilities|FlowControl|Delay _returnvalue_4)
    (CallFunction|Turnon)
    (else
      (CallFunction|Turnon)
      (Utilities|FlowControl|Delay _returnvalue_4)
      (CallFunction|TurnOff))))

(event Custom|DisableFlashing
  ;[1 1 1] 点滅停止
  (Variables|Default|SetFlashing false)
  (CallFunction|TurnOff))

(event EventBeginPlay
  (if (Variables|Default|GetAutoEnable)
    (CallFunction|EnableFlashing)))

(event EventTick
  (params (DeltaSeconds :type Float%20%28single-precision%29))
  (bind _bpm (Variables|Default|GetBPM))
  (bind _returnvalue (/ _bpm 60))
  (bind _returnvalue_2 (/ 1e+03 _returnvalue))
  (bind _returnvalue_3 (* 0.001 _returnvalue_2))
  (bind _returnvalue_4 (/ _returnvalue_3 2.0))
  ;[1 1 1] BPMに合わせて点滅
  (if (Variables|Default|GetFlashing)
    (Variables|Default|SetTime (+ DeltaSeconds (Variables|Default|GetTime)))
    (if (>= (Variables|Default|GetTime) _returnvalue_3)
      (Variables|Default|SetTime 0.0)
      (if (Variables|Default|GetDownBeat)
        (CallFunction|TurnOff)
        (Utilities|FlowControl|Delay _returnvalue_4)
        (CallFunction|Turnon)
        (else
          (CallFunction|Turnon)
          (Utilities|FlowControl|Delay _returnvalue_4)
          (CallFunction|TurnOff))))))

(fn ConstructionScript
  (bind _returnvalue (Rendering|Material|CreateDynamicMaterialInstance (Variables|Default|GetStaticMesh) 0 "/Game/Project_Omerice/BluePrints/BPMSyncedFlashing/M_BPMSyncedFlashing.M_BPMSyncedFlashing" "None" :!class /Script/Engine.PrimitiveComponent))
  (Variables|Default|SetDynamicMaterial _returnvalue))