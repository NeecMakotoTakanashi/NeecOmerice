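; BP_FloatingProp is a physics-driven prop that drifts back and forth along the world X axis around a spawn area.
; BeginPlay picks a random positive or negative X direction and gives an initial impulse; Tick keeps pushing with mass-scaled force.
; A one-second timer tests the location against the X/Y bounds supplied through Init, reversing direction once on exit, with an Outside flag preventing repeated flips.
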(event Custom|Timer
  (CallFunction|CheckState))

(event EventBeginPlay
  (Utilities|Time|SetTimerbyEvent (delegate Custom|Timer) 1.0 true)
  (Utilities|FlowControl|Sequence
    (:then_0
      (switch int (Math|Random|RandomInteger 4)
        (:0
          (Variables|Default|SetForceDirection "1.000000,0.000000,0.000000" :!label _label))
        (:1
          (Variables|Default|SetForceDirection "-1.000000,0.000000,0.000000" :!label _label_2))
        (:2
          (goto _label))
        (:3
          (goto _label_2))))
    (:then_1
      (Physics|AddImpulse (Variables|Debug|GetStaticMeshComponent) (* (Variables|Default|GetForceDirection) (Variables|Default|GetForce)) "None" true))))

(event EventTick
  (params (DeltaSeconds :type Float%20%28single-precision%29))
  (CallFunction|Update DeltaSeconds))

(fn ConstructionScript)

(fn Update
  (params (DeltaSeconds :type Float%20%28single-precision%29))
  (bind _forcedirection (Variables|Default|GetForceDirection))
  (bind _force (Variables|Default|GetForce))
  (bind _staticmeshcomponent (Variables|Debug|GetStaticMeshComponent))
  (bind _returnvalue (Physics|GetMass _staticmeshcomponent))
  (bind _returnvalue_2 (* _forcedirection _force DeltaSeconds _returnvalue))
  (Class|PrimitiveComponent|AddForceatLocation (Variables|Debug|GetStaticMeshComponent) _returnvalue_2 (Transformation|GetActorLocation) "None")
  (Physics|AddForce (Variables|Debug|GetStaticMeshComponent) _returnvalue_2 "None" false))

(fn Init
  (params (SpawnBound :type Box%20Sphere%20Bounds%20Structure))
  (Variables|Default|SetSpawnBound SpawnBound))

(fn CheckState
  (bind _inside (CallFunction|CheckOutside))
  (if (Variables|Default|GetOutside)
    (if (not _inside)
      (Variables|Default|SetOutside false))
    (elif _inside
      (Variables|Default|SetForceDirection (* (Variables|Default|GetForceDirection) -1.0))
      (Variables|Default|SetOutside true))))

(fn CheckOutside
  (bind _returnvalue (Transformation|GetActorLocation))
  (bind _spawnbound (Variables|Default|GetSpawnBound))
  (Utilities|FlowControl|Sequence
    (:then_0
      (LocalVariables|SetOrigin (.origin _spawnbound))
      (LocalVariables|SetExtent (.boxextent _spawnbound)))
    (:then_1
      (return (Math|Boolean|ORBoolean (> (.x _returnvalue) (+ (.x (LocalVariables|GetOrigin)) (.x (LocalVariables|GetExtent)))) (< (.x _returnvalue) (- (.x (LocalVariables|GetOrigin)) (.x (LocalVariables|GetExtent)))) (< (.y _returnvalue) (- (.y (LocalVariables|GetOrigin)) (.y (LocalVariables|GetExtent)))) (> (.y _returnvalue) (+ (.y (LocalVariables|GetOrigin)) (.y (LocalVariables|GetExtent)))))))))