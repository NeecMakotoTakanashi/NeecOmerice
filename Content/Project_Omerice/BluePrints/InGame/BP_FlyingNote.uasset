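; Rhythm-game note actor that flies along its direction at a set speed and is struck as a left or right note.
; The damage amount encodes the hand (below 2 is left), and only a matching hit destroys the note and reports its timing.
; Timing is graded Perfect, Good or Bad by Y distance from the perfect line, selecting the per-side Niagara effect and hit sound.
; Overlapping an actor tagged Miss reports a miss.
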(event EventTick
  (params (DeltaSeconds :type Float%20%28single-precision%29))
  (Transformation|SetActorLocation (+ (Transformation|GetActorLocation) (* (Variables|Default|GetDirection) (Variables|Default|GetSpeed) DeltaSeconds)) true false))

(event Game|Damage|EventAnyDamage
  (params (Damage :type Float%20%28single-precision%29) (DamageType :type Damage%20Type%20Object%20Reference) (InstigatedBy :type Controller%20Object%20Reference) (DamageCauser :type Actor%20Object%20Reference))
  (switch Utilities|FlowControl|Switch|SwitchonENoteType (Variables|Default|GetNoteType)
    (:NewEnumerator0
      ;[1 1 1] Damageが1がLで2がR
      (if (< Damage 2.0)
        (bind _hiteffect (CallFunction|GetHitEffect :!label _label))
        (Niagara|SpawnSystematLocation _hiteffect (Transformation|GetActorLocation))
        (CallFunction|PlayHitSE)
        (Default|CallOnHit (CallFunction|GetTiming))
        (Actor|DestroyActor)))
    (:NewEnumerator1
      (if (>= Damage 2.0)
        (goto _label)))))

(event Collision|EventActorBeginOverlap
  (params (OtherActor :type Actor%20Object%20Reference))
  (Utilities|IsValid OtherActor
    (:Is%20Valid
      (if (Actor|ActorHasTag OtherActor "Miss")
        (Default|CallOnMiss)))))

(fn ConstructionScript)

(fn SetNoteType
  (params (NoteType :type ENoteType%20Enum :default "NewEnumerator0"))
  (bind _hiteffects (Variables|Default|GetHitEffects))
  (bind _output_get (Variables|Default|SetNoteType NoteType))
  (Utilities|FlowControl|Sequence
    (:then_0
      (Utilities|Array|Clear (Variables|Default|GetHitEffects)))
    (:then_1
      (switch Utilities|FlowControl|Switch|SwitchonENoteType _output_get
        (:NewEnumerator0
          (Utilities|Array|SetArrayElem _hiteffects 0 "/Game/TeacherContent/Effects/NS_Spark_DebrisSample_Perfect_L.NS_Spark_DebrisSample_Perfect_L" true)
          (Utilities|Array|SetArrayElem _hiteffects 1 "/Game/TeacherContent/Effects/NS_Spark_DebrisSample_Good_L.NS_Spark_DebrisSample_Good_L" true)
          (Utilities|Array|SetArrayElem _hiteffects 2 "/Game/TeacherContent/Effects/NS_Spark_DebrisSample_Bad_L.NS_Spark_DebrisSample_Bad_L" true))
        (:NewEnumerator1
          (Utilities|Array|SetArrayElem _hiteffects 0 "/Game/TeacherContent/Effects/NS_Spark_DebrisSample_Perfect_R.NS_Spark_DebrisSample_Perfect_R" true)
          (Utilities|Array|SetArrayElem _hiteffects 1 "/Game/TeacherContent/Effects/NS_Spark_DebrisSample_Good_R.NS_Spark_DebrisSample_Good_R" true)
          (Utilities|Array|SetArrayElem _hiteffects 2 "/Game/TeacherContent/Effects/NS_Spark_DebrisSample_Bad_R.NS_Spark_DebrisSample_Bad_R" true))))))

(fn GetHitEffect
  (return (Utilities|Array|Get(acopy) (Variables|Default|GetHitEffects) (Math|Conversions|ToInteger(Byte) (CallFunction|GetTiming)))))

(fn GetTiming
  (bind _returnvalue (Transformation|GetActorLocation))
  (bind _perfectliney (Variables|Default|GetPerfectLineY))
  (bind _noteextent (Variables|Default|GetNoteExtent))
  (bind _returnvalue_2 (- _perfectliney (.y _returnvalue)))
  (bind _returnvalue_3 (Math|Float|Absolute(Float) _returnvalue_2))
  (if (<= _returnvalue_3 (* _noteextent 0.6))
    (return "NewEnumerator2")
    (elif (<= _returnvalue_3 _noteextent)
      (return "NewEnumerator1")
      (else
        (return "NewEnumerator0")))))

(fn PlayHitSE
  (switch Utilities|FlowControl|Switch|SwitchonENoteHitTiming (CallFunction|GetTiming)
    (:NewEnumerator2
      (LocalVariables|SetSE "/Game/Project_Omerice/SE/3_InGame/notes_perfect/SE_notes_perfect_base_01.SE_notes_perfect_base_01"))
    (:NewEnumerator1
      (LocalVariables|SetSE "/Game/Project_Omerice/SE/3_InGame/notes_good/SE_notes_good_base_01.SE_notes_good_base_01"))
    (:NewEnumerator0
      (LocalVariables|SetSE "/Game/Project_Omerice/SE/3_InGame/notes_bad/SE_notes_bad_base_02.SE_notes_bad_base_02")))
  (Audio|PlaySoundatLocation (LocalVariables|GetSE) (Transformation|GetActorLocation) "0, 0, 0" 1.0 1.0 0.0 0 0 0 0))