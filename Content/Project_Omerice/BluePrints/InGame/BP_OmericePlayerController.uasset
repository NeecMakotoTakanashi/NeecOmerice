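; Player controller that counts left clicks as score and shows the result screens.
; BeginPlay disables the pawn's collision and pre-creates the high score ranking widget.
; The R key steps through a non-looping MultiGate: personal score, then a freshly created ranking, then hidden, with no further response.
; Gamemode mob-spawn calls, a score print and some widget-swap nodes are left unconnected.
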(event EventBeginPlay
  (Utilities|FlowControl|Sequence
    (:then_0
      (Collision|SetActorEnableCollision (Game|Player|GetPlayerPawn 0) false))
    (:then_1
      ;[1 1 1] ゲーム開始時にWidgetを作成
      (Utilities|FlowControl|Sequence
        (:then_0
          (bind _returnvalue (UserInterface|CreateWidget "/Game/Project_Omerice/UI/Result_UIs_Wong/WGBP_Result_HighScoreRanking.WGBP_Result_HighScoreRanking_C"))
          (Variables|Default|SetHighScoreRanking _returnvalue))))))

(event Input|MouseEvents|LeftMouseButton
  (params (Key :type Key%20Structure))
  ;[1 1 1] カウントするノード
  (:Pressed
    (bind _output_get (Variables|Default|SetScore (+ (Variables|Default|GetScore) 1))) ; i := i + 1;
  ))

(event Input|MouseEvents|RightMouseButton
  (params (Key :type Key%20Structure)))

(event Input|KeyboardEvents|R
  (params (Key :type Key%20Structure))
  ;[1 1 1] RでリザルトUIを表示/不表示する
  (:Pressed
    (Utilities|FlowControl|MultiGate false false -1
      (:Out%200
        (UserInterface|Viewport|AddtoViewport (Variables|Default|GetMyScore) 0)
        (bind _returnvalue (UserInterface|CreateWidget "/Game/Project_Omerice/UI/Result_UIs_Wong/WGBP_Result_MyScore.WGBP_Result_MyScore_C"))
        (bind _output_get (Variables|Default|SetMyScore _returnvalue))
        (UserInterface|Viewport|AddtoViewport _output_get 0))
      (:Out%201
        (Widget|RemovefromParent (Variables|Default|GetMyScore))
        (bind _returnvalue_2 (UserInterface|CreateWidget "/Game/Project_Omerice/UI/Result_UIs_Wong/WGBP_Result_HighScoreRanking.WGBP_Result_HighScoreRanking_C"))
        (bind _output_get_2 (Variables|Default|SetHighScoreRanking _returnvalue_2))
        (UserInterface|Viewport|AddtoViewport _output_get_2 0))
      (:Out%202
        (Widget|RemovefromParent (Variables|Default|GetHighScoreRanking))))))

(event Input|MouseEvents|LeftMouseButton
  (params (Key :type Key%20Structure)))

(fn ConstructionScript)