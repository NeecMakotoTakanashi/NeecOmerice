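; Sword component that deals damage to actors it sweeps through, with the amount set by its Left or Right NoteType.
; Each tick it derives frame-rate-scaled tip velocity and an acceleration value, which must pass a threshold before hits count.
; Sphere traces at interpolated points between two blade sockets link current and cached positions, covering gaps between frames.
; PreviousVelocity is never updated here, so the acceleration check effectively follows velocity.
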(event Custom|CacheTraceLocations
  (Variables|Default|SetLastTraceStartLocation (Transformation|GetSocketLocation (Variables|Default|GetSocketNameStart)))
  (Variables|Default|SetLastTraceEndLocation (Transformation|GetSocketLocation (Variables|Default|GetSocketNameEnd))))

(event EventBeginPlay
  (Utilities|FlowControl|Sequence
    (:then_0
      (CallFunction|CacheTraceLocations)
      (Variables|Default|SetTraceStep (/ (Math|Vector|Distance(Vector) (Variables|Default|GetLastTraceStartLocation) (Variables|Default|GetLastTraceEndLocation)) 1e+01)))
    (:then_1
      (Variables|Default|SetPreviousLocation (Variables|Default|GetLastTraceEndLocation)))))

(event EventTick
  (params (DeltaSeconds :type Float%20%28single-precision%29))
  (bind _returnvalue (Components|GetOwner))
  (Utilities|FlowControl|Sequence
    (:then_0
      (CallFunction|CalcVelocity DeltaSeconds)
      (CallFunction|CalcAccelaration DeltaSeconds))
    (:then_1
      (if (CallFunction|CanSwordHit)
        (for _index (range 0 10)
          (bind _outhit (Collision|SphereTraceByChannel (Math|Vector|Lerp(Vector) (Transformation|GetSocketLocation (Variables|Default|GetSocketNameStart)) (Transformation|GetSocketLocation (Variables|Default|GetSocketNameEnd)) (/ (Math|Conversions|ToFloat(Integer) _index) 1e+01)) (Math|Vector|Lerp(Vector) (Variables|Default|GetLastTraceStartLocation) (Variables|Default|GetLastTraceEndLocation) (/ (Math|Conversions|ToFloat(Integer) _index) 1e+01)) (Variables|Default|GetTraceStep) "TraceTypeQuery1" false 0 "None" true "(R=1.000000,G=0.000000,B=0.000000,A=1.000000)" "(R=0.000000,G=1.000000,B=0.000000,A=1.000000)" 0.2))
          (Utilities|IsValid (.HitActor (Collision|BreakHitResult _outhit))
            (:Is%20Valid
              (switch Utilities|FlowControl|Switch|SwitchonENoteType (Variables|Default|GetNoteType)
                (:NewEnumerator0
                  (Game|Damage|ApplyDamage (.HitActor (Collision|BreakHitResult _outhit)) 1.0 0 _returnvalue))
                (:NewEnumerator1
                  (Game|Damage|ApplyDamage (.HitActor (Collision|BreakHitResult _outhit)) 2.0 0 _returnvalue)))))))
      (CallFunction|CacheTraceLocations))))

(fn CalcVelocity
  (params (DeltaSeconds :type Float%20%28double-precision%29))
  (bind _lasttraceendlocation (Variables|Default|GetLastTraceEndLocation))
  (Variables|Default|SetCurrentVelocity (* (- _lasttraceendlocation (Variables|Default|GetPreviousLocation)) (* DeltaSeconds (Variables|Default|GetTargetFPS))))
  (Variables|Default|SetPreviousLocation _lasttraceendlocation))

(fn CalcAccelaration
  (params (DeltaSeconds :type Float%20%28double-precision%29))
  (bind _output_get (Variables|Default|SetCurrentAccelaration (- (Variables|Default|GetCurrentVelocity) (Variables|Default|GetPreviousVelocity)))))

(fn CanSwordHit
  (return (>= (Math|Vector|VectorLengthSquared (Variables|Default|GetCurrentAccelaration)) (Variables|Default|GetAccelarationThresholdSquared))))