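; Test laser sword actor that damages whatever its blade touches, using per-tick sphere traces on the Visibility channel.
; Traces are spaced between the TraceStart and TraceEnd sockets, with radius derived from blade length at BeginPlay.
; Socket positions are re-cached after each trace, so only the first sweeps from last tick's position.
; Every trace hit applies fixed damage, with no duplicate filtering.
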(event Custom|CacheTraceLocations
  (bind _staticmeshcomponent (Variables|Debug|GetStaticMeshComponent))
  (Variables|Default|SetLastTraceStartLocation (Transformation|GetSocketLocation _staticmeshcomponent "TraceStart"))
  (Variables|Default|SetLastTraceEndLocation (Transformation|GetSocketLocation _staticmeshcomponent "TraceEnd")))

(event EventBeginPlay
  (CallFunction|CacheTraceLocations)
  (Variables|Default|SetTraceStep (/ (Math|Vector|Distance(Vector) (Variables|Default|GetLastTraceStartLocation) (Variables|Default|GetLastTraceEndLocation)) 2e+01)))

(event EventTick
  (params (DeltaSeconds :type Float%20%28single-precision%29))
  (bind _staticmeshcomponent (Variables|Debug|GetStaticMeshComponent))
  (for _index (range 0 10)
    (bind _outhit (Collision|SphereTraceByChannel (Math|Vector|Lerp(Vector) (Transformation|GetSocketLocation _staticmeshcomponent "TraceStart") (Transformation|GetSocketLocation _staticmeshcomponent "TraceEnd") (/ (Math|Conversions|ToFloat(Integer) _index) 1e+01)) (Math|Vector|Lerp(Vector) (Variables|Default|GetLastTraceStartLocation) (Variables|Default|GetLastTraceEndLocation) (/ (Math|Conversions|ToFloat(Integer) _index) 1e+01)) (Variables|Default|GetTraceStep) "TraceTypeQuery1" false 0 "None" true "(R=1.000000,G=0.000000,B=0.000000,A=1.000000)" "(R=0.000000,G=1.000000,B=0.000000,A=1.000000)" 0.2))
    (CallFunction|CacheTraceLocations)
    (Utilities|IsValid (.HitActor (Collision|BreakHitResult _outhit))
      (:Is%20Valid
        (Game|Damage|ApplyDamage (.HitActor (Collision|BreakHitResult _outhit)) 1e+02 0 self)))))

(fn ConstructionScript)