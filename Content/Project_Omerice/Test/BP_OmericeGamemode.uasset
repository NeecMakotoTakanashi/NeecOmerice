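; Test game mode for Omerice that spawns flying notes in front of the PlayerStart and prints Combo or Miss from their callbacks.
; BeginPlay caches the spawn centre, then BPISpawnNotes picks a left or right mesh and maps NoteID to a 3x3 grid offset on world X/Z.
; Also holds helpers, uncalled in this graph, for camera raycasts and mob spawning by random drop, impulse launch or unique floor-grid cell.
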(event Custom|OnMiss
  (Development|PrintString "Miss"))

(event Custom|OnHit
  (Development|PrintString "Combo"))

(event EventBeginPlay
  (CallFunction|SetNoteSpawnLocation))

(event EventBPISpawnNotes
  (params (NoteType :type ENoteType%20Enum :default "NewEnumerator0") (NoteID :type Integer))
  (bind _spawnnote (CallFunction|SpawnNote NoteType NoteID))
  (EventDispatchers|BindEventtoOnHit _spawnnote (delegate Custom|OnHit))
  (EventDispatchers|BindEventtoOnMiss _spawnnote (delegate Custom|OnMiss)))

(fn ConstructionScript)

(fn GetRaycastLocation
  (bind _returnvalue (Game|GetPlayerCameraManager 0))
  (bind _returnvalue_2 (Camera|GetCameraLocation _returnvalue))
  (bind (_outhit _returnvalue_3) (Collision|LineTraceByChannel _returnvalue_2 (+ _returnvalue_2 (* (Math|Vector|GetForwardVector (Camera|GetCameraRotation _returnvalue)) 1.5e+03)) "TraceTypeQuery1" false 0 "ForOneFrame"))
  (return _returnvalue_3 (.Location (Collision|BreakHitResult _outhit))))

(fn SpawnActor
  (params (Transform :type Transform))
  (bind _returnvalue (Game|SpawnActorfromClass (Variables|Default|GetMobActorClass) Transform "Undefined" 0 0))
  (bind _asbp_physics_actor (Utilities|Casting|CastToBP_PhysicsActor _returnvalue)
    (:then
      _)
    (:CastFailed
      _))
  (return (Variables|/Script/Engine.StaticMeshActor|GetStaticMeshComponent _asbp_physics_actor)))

(fn SpawnMobFall
  (CallFunction|SpawnActor (Math|Transform|MakeTransform (Math|Vector|MakeVector (Math|Random|RandomFloatinRange 6.2e+02 1.45e+03) (Math|Random|RandomFloatinRange -8.8e+02 6.6e+02) 8e+02))))

(fn SpawnMobLaunch
  (params (PlayerStart :type Actor%20Object%20Reference))
  (bind _mobimpluse (Variables|Default|GetMobImpluse))
  (bind _spawnwideangle (Variables|Default|GetSpawnWideAngle))
  (bind _spawntileangle (Variables|Default|GetSpawnTileAngle))
  (bind _staticmesh (CallFunction|SpawnActor (Math|Transform|MakeTransform (.location (Transformation|GetActorTransform PlayerStart)))))
  (Physics|AddImpulse _staticmesh (* (Math|Vector|RotateVector (Math|Vector|RotateVector "1.000000,0.000000,0.000000" (Math|Rotator|MakeRotator 0.0 (Math|Random|RandomFloatinRange (* _spawntileangle -1.0) _spawntileangle) 0.0)) (Math|Rotator|MakeRotator 0.0 1e+01 (+ (.Yaw (Math|Rotator|BreakRotator (Math|Rotator|MakeRotfromX (Transformation|GetActorForwardVector PlayerStart)))) (Math|Random|RandomFloatinRange (* _spawnwideangle -1.0) _spawnwideangle)))) (Math|Random|RandomFloatinRange _mobimpluse (* _mobimpluse (Variables|Default|GetMobImpluseMaxScale)))) "None" true))

(fn SpawnMobFloor
  (bind _occupaid (Variables|Default|GetOccupaid))
  (bind _output_get (LocalVariables|SetSpawnGrid (Utilities|Struct|MakeIntPoint (Math|Random|RandomIntegerinRange 0 8) (Math|Random|RandomIntegerinRange 0 15))))
  (if (== (Utilities|Array|FindItem _occupaid _output_get) -1)
    (Utilities|Array|Add _occupaid (LocalVariables|GetSpawnGrid))
    (CallFunction|SpawnActor (Math|Transform|MakeTransform (Math|Vector|MakeVector (Math|Conversions|ToFloat(Integer) (+ 615 (* (.x (LocalVariables|GetSpawnGrid)) 113))) (Math|Conversions|ToFloat(Integer) (- 544 (* (.y (LocalVariables|GetSpawnGrid)) 100))) 2.0)))))

(fn GetNoteOffset
  (params (Type :type Integer))
  (return ""))

(fn SpawnNote
  (params (NoteType :type ENoteType%20Enum :default "NewEnumerator0") (NoteID :type Integer))
  (bind _notespawnlocaloffset (Variables|Default|GetNoteSpawnLocalOffset))
  (Utilities|FlowControl|Sequence
    (:then_0
      (switch Utilities|FlowControl|Switch|SwitchonENoteType NoteType
        (:NewEnumerator0
          (LocalVariables|SetSpawnMesh (Variables|Default|GetSM_NoteL)))
        (:NewEnumerator1
          (LocalVariables|SetSpawnMesh (Variables|Default|GetSM_NoteR)))))
    (:then_1
      (Variables|Default|SetNoteSpawnNormalizedPosition (CallFunction|GetSpawnNormalizedPositionfromID NoteID)))
    (:then_2
      (bind _returnvalue (Game|SpawnActorfromClass "/Game/Project_Omerice/Test/SaberTest/BP_FlyingNote.BP_FlyingNote_C" (Math|Transform|MakeTransform (+ (Variables|Default|GetNoteSpawnLocation) (Math|Vector|MakeVector (* (.x (Variables|Default|GetNoteSpawnNormalizedPosition)) _notespawnlocaloffset) 0.0 (* _notespawnlocaloffset (.z (Variables|Default|GetNoteSpawnNormalizedPosition))))) "0, 0, 0" "1.000000,1.000000,1.000000") "AlwaysSpawn" 0 0))
      (Components|StaticMesh|SetStaticMesh (Variables|/Script/Engine.StaticMeshActor|GetStaticMeshComponent _returnvalue) (LocalVariables|GetSpawnMesh))
      (return _returnvalue))))

(fn GetSpawnNormalizedPositionfromID
  (params (NoteID :type Integer))
  (switch int NoteID
    (:Default
      _)
    (:0
      _)
    (:1
      (return (Utilities|Struct|MakeIntVector -1 0 1)))
    (:2
      (return (Utilities|Struct|MakeIntVector 0 0 1)))
    (:3
      (return (Utilities|Struct|MakeIntVector 1 0 1)))
    (:4
      (return (Utilities|Struct|MakeIntVector -1 0 0)))
    (:5
      _)
    (:6
      (return (Utilities|Struct|MakeIntVector 1 0 0)))
    (:7
      (return (Utilities|Struct|MakeIntVector -1 0 -1)))
    (:8
      (return (Utilities|Struct|MakeIntVector 0 0 -1)))
    (:9
      (return (Utilities|Struct|MakeIntVector 1 0 -1))))
  (return (Utilities|Struct|MakeIntVector 0 0 0)))

(fn SetNoteSpawnLocation
  (bind _returnvalue (Actor|GetActorOfClass "/Script/Engine.PlayerStart"))
  (Variables|Default|SetNoteSpawnLocation (+ (Transformation|GetActorLocation _returnvalue) (* (Transformation|GetActorForwardVector _returnvalue) (CallFunction|GetNoteSpawnOffsetfromPlayerStart)) (Math|Vector|MakeVector 0.0 0.0 (* (Variables|Default|GetNoteSpawnLocalOffset) 2.0)))))

(fn GetNoteSpawnOffsetfromPlayerStart
  (return 1.3e+03))