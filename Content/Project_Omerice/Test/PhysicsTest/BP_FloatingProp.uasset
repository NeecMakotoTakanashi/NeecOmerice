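; BP_FloatingProp is a physics test prop that gets pushed continuously in a random horizontal direction.
; On BeginPlay it picks one of the four positive or negative X and Y world axes as its force direction.
; Every Tick it applies that direction, scaled by a Force variable, to its static mesh component at the actor's location.
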(event EventBeginPlay
  (switch int (Math|Random|RandomInteger 4)
    (:0
      (Variables|Default|SetForceDirection "1.000000,0.000000,0.000000"))
    (:1
      (Variables|Default|SetForceDirection "-1.000000,0.000000,0.000000"))
    (:2
      (Variables|Default|SetForceDirection "0.000000,1.000000,0.000000"))
    (:3
      (Variables|Default|SetForceDirection "0.000000,-1.000000,0.000000"))))

(event Collision|EventActorBeginOverlap
  (params (OtherActor :type Actor%20Object%20Reference)))

(event EventTick
  (params (DeltaSeconds :type Float%20%28single-precision%29))
  (Class|PrimitiveComponent|AddForceatLocation (Variables|Debug|GetStaticMeshComponent) (* (Variables|Default|GetForceDirection) (Variables|Default|GetForce)) (Transformation|GetActorLocation) "None"))

(fn ConstructionScript)