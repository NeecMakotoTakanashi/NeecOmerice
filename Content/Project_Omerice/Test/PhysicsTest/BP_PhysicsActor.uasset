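; BP_PhysicsActor is a test actor that grows from a reduced scale to its placed size as it ages.
; On BeginPlay it stores the actor's scale and the static mesh's linear damping as targets, then multiplies both by StartScalePercentage for starting values.
; Tick accumulates Age and, until TargetAge, lerps scale and damping back to their targets through the shared ScaleCurve.
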(event EventBeginPlay
  (CallFunction|Initialize))

(event Collision|EventActorBeginOverlap
  (params (OtherActor :type Actor%20Object%20Reference)))

(event EventTick
  (params (DeltaSeconds :type Float%20%28single-precision%29))
  (CallFunction|Update DeltaSeconds))

(fn ConstructionScript)

(fn Initialize
  (bind _returnvalue (Transformation|GetActorScale3D))
  (bind _staticmeshcomponent (Variables|Debug|GetStaticMeshComponent))
  (bind _returnvalue_2 (Class|PrimitiveComponent|GetLinearDamping _staticmeshcomponent))
  (Utilities|FlowControl|Sequence
    (:then_0
      (Variables|Default|SetTargetScale _returnvalue)
      (bind _output_get (Variables|Default|SetStartScale (* _returnvalue (Variables|Default|GetStartScalePercentage))))
      (Transformation|SetActorScale3D _output_get))
    (:then_1
      (Variables|Default|SetTargetLinearDamping _returnvalue_2)
      (bind _output_get_2 (Variables|Default|SetStartLinearDamping (* _returnvalue_2 (Variables|Default|GetStartScalePercentage))))
      (Class|PrimitiveComponent|SetLinearDamping _staticmeshcomponent _output_get_2))))

(fn Update
  (params (DeltaTime :type Float%20%28double-precision%29))
  (Utilities|FlowControl|Sequence
    (:then_0
      (if (<= (Variables|Default|GetAge) (Variables|Default|GetTargetAge))
        (Transformation|SetActorScale3D (Math|Vector|Lerp(Vector) (Variables|Default|GetStartScale) (Variables|Default|GetTargetScale) (Math|Curves|GetFloatValue (Variables|Default|GetScaleCurve) (Math|Float|Clamp(Float) (/ (Variables|Default|GetAge) (Variables|Default|GetTargetAge))))))
        (Class|PrimitiveComponent|SetLinearDamping (Variables|Debug|GetStaticMeshComponent) (Math|Float|Lerp (Variables|Default|GetStartLinearDamping) (Variables|Default|GetTargetLinearDamping) (Math|Curves|GetFloatValue (Variables|Default|GetScaleCurve) (Math|Float|Clamp(Float) (/ (Variables|Default|GetAge) (Variables|Default|GetTargetAge))))))))
    (:then_1
      (Variables|Default|SetAge (+ DeltaTime (Variables|Default|GetAge))))))