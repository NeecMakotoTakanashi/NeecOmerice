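; Menu actor for picking one of six music genres, then showing that genre's song list.
; Test left/right inputs step a clamped index and highlight that genre with a timeline-driven emissive dynamic material.
; OK hides the other genres, eases the chosen one along Y toward AnimPosition, and reveals the song panel.
; The panel is tinted per genre and hides surplus song slots using enum entry counts; Back is unfinished.
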(event Custom|Genre_Select
  (bind _genre_objects_array (Variables|Default|GetGenre_Objects_Array))
  (bind _action_material (Variables|Default|GetAction_Material))
  ;[1 1 1] Select_Effect
  (Rendering|Material|SetMaterial _genre_objects_array 0 _action_material)
  (bind _returnvalue (Rendering|Material|CreateDynamicMaterialInstance (Utilities|Array|Get(acopy) _genre_objects_array (Variables|Default|GetFix_Genre_Numver)) 0 _action_material "" :!class /Script/Engine.PrimitiveComponent))
  (Rendering|Material|SetVectorParameterValue _returnvalue "Emissive_Color" "(R=1.000000,G=0.000000,B=0.000000,A=1.000000)" :!class /Script/Engine.MaterialInstanceDynamic)
  (bind _anim (Timeline|タイムライン PlayFromStart)
    (:Update
      (Rendering|Material|SetScalarParameterValue _returnvalue "Emissive" _anim :!class /Script/Engine.MaterialInstanceDynamic))))

(event Custom|Genre_OK
  (bind _fix_genre_numver (Variables|Default|GetFix_Genre_Numver))
  (bind _ganre_01_kawaii (Variables|Default|GetGanre_01_Kawaii))
  (bind _ganre_02_space (Variables|Default|GetGanre_02_Space))
  (bind _ganre_04_halloween (Variables|Default|GetGanre_04_Halloween))
  (bind _ganre_05_summer (Variables|Default|GetGanre_05_Summer))
  (bind _ganre_06_park (Variables|Default|GetGanre_06_Park))
  (bind _ganre_03_school (Variables|Default|GetGanre_03_School))
  (bind _array (Utilities|Array|MakeArray _ganre_01_kawaii _ganre_02_space _ganre_03_school _ganre_04_halloween _ganre_05_summer _ganre_06_park))
  (bind _output (Utilities|Array|Get(acopy) _array _fix_genre_numver))
  ;[1 1 1] Select_Object_Hidd
  (for (_array_element _array_index) (Variables|Default|GetGenre_Objects_Array)
    (if (!= _array_index (Variables|Default|GetFix_Genre_Numver))
      (Development|SetHiddeninGame _array_element true false)
      ;[1 1 1] Genre_Object_Anim
      (Timeline|タイムライン_0 Play
        (:Update
          (Transformation|AddWorldOffset _output (Math|Vector|MakeVector 0.0 (Math|Float|Lerp 0.0 (- (.y (Transformation|GetWorldLocation (Variables|Default|GetAnim_Position))) (.y (Transformation|GetWorldLocation _output))) 0.1) 0.0) false false)
          (CallFunction|SongSelect))))))

(event Custom|Song_Select
  (bind _song_menu_00 (Variables|Default|GetSong_Menu_00))
  (bind _songs_array (Variables|Default|GetSongs_Array))
  (bind _songs_kawaii (Variables|Default|GetSongs_Kawaii))
  (bind _fix_genre_numver (Variables|Default|GetFix_Genre_Numver))
  (bind _m_genremenu (Variables|Default|GetM_GenreMenu))
  (bind _returnvalue (- _songs_kawaii 1))
  (bind _returnvalue_2 (Math|Integer|Clamp(Integer) _fix_genre_numver 0 _returnvalue))
  (bind _output (Utilities|Array|Get(acopy) _songs_array _returnvalue_2))
  (bind _returnvalue_3 (Transformation|GetWorldLocation _output))
  ;[1 1 1] Menuモデル表示_識別テスト
  (Development|SetHiddeninGame (Variables|Default|GetSongs_Objects_Array) false false)
  (Rendering|Material|SetMaterial _song_menu_00 0 _m_genremenu)
  (bind _returnvalue_4 (Rendering|Material|CreateDynamicMaterialInstance _song_menu_00 0 _m_genremenu "None" :!class /Script/Engine.PrimitiveComponent))
  (Rendering|Material|SetVectorParameterValue _returnvalue_4 "TestColor" (Utilities|Array|Get(acopy) (Utilities|Array|MakeArray "(R=1.000000,G=0.183333,B=0.360277,A=1.000000)" "(R=0.000000,G=0.233333,B=1.000000,A=1.000000)" "(R=1.000000,G=0.186363,B=0.000000,A=1.000000)" "(R=0.433333,G=0.000000,B=1.000000,A=1.000000)" "(R=1.000000,G=0.016463,B=0.000000,A=1.000000)" "(R=0.022268,G=1.000000,B=0.000000,A=1.000000)") (Variables|Default|GetFix_Genre_Numver)) :!class /Script/Engine.MaterialInstanceDynamic)
  (switch int (Variables|Default|GetFix_Genre_Numver)
    (:0
      ;[1 1 1] ジャンルごとの曲数に合わせた表示
      (for _index (range (Variables|Default|GetSongs_Kawaii) (Variables|Default|GetSong_MaxItem))
        (Development|SetHiddeninGame (Utilities|Array|Get(acopy) (Variables|Default|GetSongs_Array) _index) true false)
        ;[1 1 1] １つ１つのオブジェクトのスケールとかを変更させたかった
        (Transformation|SetWorldTransform _output (Math|Transform|MakeTransform (Math|Vector|MakeVector (.x _returnvalue_3) (.y _returnvalue_3) 1e+01) "0, 0, 0" (Variables|Default|GetSong_Name_Transform_Scale)) false false)))
    (:1
      (for _index_2 (range (Variables|Default|GetSong_Space) (Variables|Default|GetSong_MaxItem))
        (Development|SetHiddeninGame (Utilities|Array|Get(acopy) (Variables|Default|GetSongs_Array) _index_2) true false)))
    (:2
      (for _index_3 (range (Variables|Default|GetSongs_School) (Variables|Default|GetSong_MaxItem))
        (Development|SetHiddeninGame (Utilities|Array|Get(acopy) (Variables|Default|GetSongs_Array) _index_3) true false)))
    (:3
      (for _index_4 (range (Variables|Default|GetSong_Halloween) (Variables|Default|GetSong_MaxItem))
        (Development|SetHiddeninGame (Utilities|Array|Get(acopy) (Variables|Default|GetSongs_Array) _index_4) true false)))
    (:4
      (for _index_5 (range (Variables|Default|GetSong_Summer) (Variables|Default|GetSong_MaxItem))
        (Development|SetHiddeninGame (Utilities|Array|Get(acopy) (Variables|Default|GetSongs_Array) _index_5) true false)))
    (:5
      (for _index_6 (range (Variables|Default|GetSong_Park) (Variables|Default|GetSong_MaxItem))
        (Development|SetHiddeninGame (Utilities|Array|Get(acopy) (Variables|Default|GetSongs_Array) _index_6) true false)))))

(event EventBeginPlay
  (bind _song_name_00 (Variables|Default|GetSong_Name_00))
  (bind _ganre_02_space (Variables|Default|GetGanre_02_Space))
  (bind _ganre_04_halloween (Variables|Default|GetGanre_04_Halloween))
  (bind _ganre_05_summer (Variables|Default|GetGanre_05_Summer))
  (bind _ganre_06_park (Variables|Default|GetGanre_06_Park))
  (bind _ganre_03_school (Variables|Default|GetGanre_03_School))
  (bind _song_name_04 (Variables|Default|GetSong_Name_04))
  (bind _song_name_03 (Variables|Default|GetSong_Name_03))
  (bind _song_name_02 (Variables|Default|GetSong_Name_02))
  (bind _song_name_01 (Variables|Default|GetSong_Name_01))
  (bind _ganre_01_kawaii (Variables|Default|GetGanre_01_Kawaii))
  (bind _array (Utilities|Array|MakeArray _ganre_01_kawaii _ganre_02_space _ganre_03_school _ganre_04_halloween _ganre_05_summer _ganre_06_park))
  (bind _array_2 (Utilities|Array|MakeArray _song_name_00 _song_name_01 _song_name_02 _song_name_03 _song_name_04))
  ;[1 1 1] コメント
  (Utilities|FlowControl|Sequence
    (:then_0
      (Input|EnableInput (Game|GetPlayerController 0))
      ;[1 1 1] 現在のジャンル数
      (Variables|Default|SetGenre_MaxItem (Utilities|Array|Length _array))
      ;[1 1 1] 全オブジェクト呼び出し
      (Variables|Default|SetGenre_Objects_Array _array)
      ;[1 1 1] オブジェクト指定
      (Variables|Default|SetSelect_Genre_Object (Utilities|Array|Get(acopy) _array))
      ;[1 1 1] 曲選択画面全オブジェクト
      (bind _output_get (Variables|Default|SetSongs_Objects_Array (Utilities|Array|MakeArray (Variables|Default|GetSong_Name_Genre) (Variables|Default|GetSong_Menu_00) (Variables|Default|GetSong_Back_for_Genre) _song_name_00 _song_name_01 _song_name_02 _song_name_03 _song_name_04)))
      (Development|SetHiddeninGame _output_get true false)
      ;[1 1 1] 全曲
      (Variables|Default|SetSongs_Array _array_2)
      ;[1 1 1] 曲を選ぶ
      (Variables|Default|Setselect_Song_Name (Utilities|Array|Get(acopy) _array_2 (Math|Integer|Clamp(Integer) (Variables|Default|GetFix_Genre_Numver) 3 0)))
      ;[1 1 1] 全曲数
      (Variables|Default|SetSong_MaxItem (Utilities|Array|Length _array_2))
      ;[1 1 1] 各ジャンルの曲数
      (Variables|Default|SetSongs_Kawaii (|GetNumEnumEntries))
      (Variables|Default|SetSong_Space (|GetNumEnumEntries))
      (Variables|Default|SetSongs_School (|GetNumEnumEntries))
      (Variables|Default|SetSong_Halloween (|GetNumEnumEntries))
      (Variables|Default|SetSong_Summer (|GetNumEnumEntries))
      (Variables|Default|SetSong_Park (|GetNumEnumEntries)))
    (:then_1
      (if (Variables|Default|GetIn_Controller)
        _))))

(event Collision|EventActorBeginOverlap
  (params (OtherActor :type Actor%20Object%20Reference)))

(event EventTick
  (params (DeltaSeconds :type Float%20%28single-precision%29)))

(event Input|ActionEvents|InputActionTest_OK
  (params (Key :type Key%20Structure :default "None"))
  ;[1 1 1] OK
  (:Pressed
    (Variables|Default|SetIn_OK true)
    (Utilities|FlowControl|DoOnce false
      (:Completed
        (CallFunction|GenreOK)
        (Development|PrintString "Genre_OK" true true "(R=1.000000,G=0.000000,B=0.000000,A=1.000000)"))))
  (:Released
    (Variables|Default|SetIn_OK false)))

(event Input|ActionEvents|InputActionTest_Back
  (params (Key :type Key%20Structure :default "None"))
  ;[1 1 1] Back
  (:Pressed
    (Variables|Default|SetIn_Back true))
  (:Released
    (Variables|Default|SetIn_Back false)))

(event Input|ActionEvents|InputActionTest_Debug
  (params (Key :type Key%20Structure :default "None"))
  (:Pressed
    (Development|PrintString "Hello" true true "(R=1.000000,G=0.000000,B=0.036246,A=1.000000)")))

(event Input|ActionEvents|InputActionTest_Right
  (params (Key :type Key%20Structure :default "None"))
  (bind _in_ok (Variables|Default|GetIn_OK))
  (bind _returnvalue (== _in_ok true))
  ;[1 1 1] ボタン入力
  (:Pressed
    (bind _output_get (Variables|Default|SetGanre_Number (Math|Integer|Clamp(Integer) (+ 1 (Variables|Default|GetGanre_Number)) 0 (- (Variables|Default|GetGenre_MaxItem) 1))))
    (bind _output_get_2 (Variables|Default|SetFix_Genre_Numver _output_get))
    (Development|PrintString (Utilities|String|ToString(Integer) _output_get_2))
    (if _returnvalue
      ;[1 1 1] Genre選択終了処理
      (CallFunction|GenreSelect)
      (else
        (Utilities|FlowControl|DoOnce _returnvalue
          (:Completed
            (CallFunction|GenreSelect)))))))

(event Input|ActionEvents|InputActionTest_Left
  (params (Key :type Key%20Structure :default "None"))
  (bind _in_ok (Variables|Default|GetIn_OK))
  (bind _returnvalue (== _in_ok true))
  ;[1 1 1] ボタン入力
  (:Pressed
    (bind _output_get (Variables|Default|SetGanre_Number (Math|Integer|Clamp(Integer) (+ -1 (Variables|Default|GetGanre_Number)) 0 (- (Variables|Default|GetGenre_MaxItem) 1))))
    (Variables|Default|SetFix_Genre_Numver _output_get)
    (Development|PrintString (Utilities|String|ToString(Integer) (stale Input|ActionEvents|InputActionTest_Right _output_get_2)))
    (if _returnvalue
      ;[1 1 1] Genre選択終了処理
      (CallFunction|GenreSelect)
      (else
        (Utilities|FlowControl|DoOnce _returnvalue
          (:Completed
            (CallFunction|GenreSelect)))))))

(fn ConstructionScript
  (Development|SetHiddeninGame (Variables|Default|GetAnim_Position) (Variables|Default|GetHIdden_In_Games) false))