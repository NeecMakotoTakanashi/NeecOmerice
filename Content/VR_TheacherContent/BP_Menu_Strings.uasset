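; Prototype genre selection menu actor in the VR teacher content, with six genre models and a glowing material for the selected one.
; BeginPlay enables player input, and left/right actions step a clamped genre index that is printed to screen.
; The construction script applies the highlight material and sets MPC emissive; input does not update the highlight.
; The index switch, controller check and Go action are stubs or debug prints.
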(event EventBeginPlay
  ;[1 1 1] ボタン操作有効
  (Utilities|FlowControl|Sequence
    (:then_0
      (Input|EnableInput (Game|GetPlayerController 0)))
    (:then_1
      (if (Variables|Default|GetIn_Controller)
        _))))

(event Collision|EventActorBeginOverlap
  (params (OtherActor :type Actor%20Object%20Reference)))

(event EventTick
  (params (DeltaSeconds :type Float%20%28single-precision%29)))

(event Input|ActionEvents|InputActionTest_Right
  (params (Key :type Key%20Structure :default "None"))
  ;[1 1 1] ジャンル番号+１
  (:Pressed
    (bind _output_get (Variables|Default|SetGanre_Numver (Math|Integer|Clamp(Integer) (+ 1 (Variables|Default|GetGanre_Numver)) 0 5)))
    (bind _output_get_2 (Variables|Default|SetFix_Ganre_Numver _output_get))
    (Development|PrintString (Utilities|String|ToString(Integer) _output_get_2))
    (switch int (Variables|Default|GetFix_Ganre_Numver)
      (:0
        (if true
          _)))))

(event Input|ActionEvents|InputActionTest_Debug
  (params (Key :type Key%20Structure :default "None"))
  ;[1 1 1] 現在選択しているジャンル番号
  (:Pressed
    (Development|PrintString (Utilities|String|ToString(Integer) (Variables|Default|GetFix_Ganre_Numver)) true true "(R=1.000000,G=0.000000,B=0.005305,A=1.000000)")))

(event Input|ActionEvents|InputActionTest_Left
  (params (Key :type Key%20Structure :default "None"))
  ;[1 1 1] ジャンル番号-1
  (:Pressed
    (bind _output_get (Variables|Default|SetGanre_Numver (Math|Integer|Clamp(Integer) (+ -1 (Variables|Default|GetGanre_Numver)) 0 5)))
    (Variables|Default|SetFix_Ganre_Numver _output_get)
    ;[1 1 1] ジャンル番号+１
    (Development|PrintString (Utilities|String|ToString(Integer) (stale Input|ActionEvents|InputActionTest_Right _output_get_2)))
    (switch int (Variables|Default|GetFix_Ganre_Numver)
      (:0
        (if true
          _)))))

(event Input|ActionEvents|InputActionGo_01
  (params (Key :type Key%20Structure :default "None"))
  (:Pressed
    (Development|PrintString "Hello")))

(fn ConstructionScript
  ;[1 1 1] 選択すると光るマテリアル
  (Rendering|Material|SetMaterial (Utilities|Array|Get(acopy) (Utilities|Array|MakeArray (Variables|Default|GetGanre_01) (Variables|Default|GetGanre_02) (Variables|Default|GetGanre_03) (Variables|Default|GetGanre_04) (Variables|Default|GetGanre_05) (Variables|Default|GetGanre_06)) (Variables|Default|GetFix_Ganre_Numver)) 0 (Variables|Default|GetAction_Material))
  (Rendering|Material|SetScalarParameterValue "/Game/VR_TheacherContent/Menu/MPC_TestMenuUI.MPC_TestMenuUI" "Emissive" 1e+01 :!class /Script/Engine.KismetMaterialLibrary))