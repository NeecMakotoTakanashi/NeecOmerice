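; Sliceable cube actor for a VR saber rhythm game that shows a cube being cut, then destroys itself.
; Slice_HIt colors the static mesh red or blue, while Slice_Miss makes it bright white.
; Both copy it to a procedural mesh and slice it along the given plane with a white cap.
; The sliced piece gets physics and a reversed impulse before the actor is destroyed after a short delay.
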(event Custom|Slice_Miss
  (params (PlanePosition :type Vector) (Impulse :type Vector) (PlaneNormal :type Vector) (IsRed :type Boolean))
  (bind _returnvalue (* Impulse -1.0))
  (bind (_x _y _z) (Math|Vector|BreakVector _returnvalue))
  (Rendering|Material|SetMaterial (Variables|Default|GetStaticMesh) 0 (select IsRed "/Game/VR_SaberRhythmGame/Materials/WhiteBright_M_Inst.WhiteBright_M_Inst" "/Game/VR_SaberRhythmGame/Materials/WhiteBright_M_Inst.WhiteBright_M_Inst"))
  (Class|KismetProceduralMeshLibrary|CopyProceduralMeshfromStaticMeshComponent (Variables|Default|GetStaticMesh) 0 (Variables|Default|GetProceduralMesh) true)
  (bind _outotherhalfprocmesh (Class|KismetProceduralMeshLibrary|SliceProceduralMesh (Variables|Default|GetProceduralMesh) PlanePosition PlaneNormal true "CreateNewSectionForCap" "/Game/VR_SaberRhythmGame/Materials/WhiteBright_M.WhiteBright_M"))
  (Collision|SetCollisionEnabled _outotherhalfprocmesh "PhysicsOnly")
  (Physics|SetSimulatePhysics _outotherhalfprocmesh true)
  (Physics|AddImpulse _outotherhalfprocmesh (Math|Vector|MakeVector _x _y _z) "None" false)
  (Utilities|FlowControl|Delay 0.3)
  (Actor|DestroyActor))

(event Custom|Slice_HIt
  (params (PlanePosition :type Vector) (Impulse :type Vector) (PlaneNormal :type Vector) (IsRed :type Boolean))
  (bind _returnvalue (* Impulse -1.0))
  (bind (_x _y _z) (Math|Vector|BreakVector _returnvalue))
  (Rendering|Material|SetMaterial (Variables|Default|GetStaticMesh) 0 (select IsRed "/Game/VR_SaberRhythmGame/Materials/Red_M.Red_M" "/Game/VR_SaberRhythmGame/Materials/Blue_M.Blue_M"))
  (Class|KismetProceduralMeshLibrary|CopyProceduralMeshfromStaticMeshComponent (Variables|Default|GetStaticMesh) 0 (Variables|Default|GetProceduralMesh) true)
  (bind _outotherhalfprocmesh (Class|KismetProceduralMeshLibrary|SliceProceduralMesh (Variables|Default|GetProceduralMesh) PlanePosition PlaneNormal true "CreateNewSectionForCap" "/Game/VR_SaberRhythmGame/Materials/WhiteBright_M.WhiteBright_M"))
  (Collision|SetCollisionEnabled _outotherhalfprocmesh "PhysicsOnly")
  (Physics|SetSimulatePhysics _outotherhalfprocmesh true)
  (Physics|AddImpulse _outotherhalfprocmesh (Math|Vector|MakeVector _x _y _z) "None" false)
  (Utilities|FlowControl|Delay 0.3)
  (Actor|DestroyActor))

(fn ConstructionScript)