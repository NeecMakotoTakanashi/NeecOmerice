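; VR menu actor for the saber rhythm game, hosting a widget that stays usable while the game is paused.
; BeginPlay caches the VR character and makes the widget tickable when paused, and Tick rotates it to face the player camera.
; Its events play or stop a passed-in song target, and Unpause tells the character to resume, then destroys the menu.
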(event Custom|PlaySong
  (params (Target :type Audio%20Component%20Object%20Reference))
  (Audio|Components|Audio|Play Target 0.0))

(event Custom|StopSong
  (params (Target :type Audio%20Component%20Object%20Reference))
  (Audio|Components|Audio|Stop Target))

(event Custom|Unpause
  (Default|Unpause (Variables|Default|GetBP_VRCharacter_Ref))
  (Actor|DestroyActor))

(event EventBeginPlay
  (bind _asbp_vrcharacter (Utilities|Casting|CastToBP_VRCharacter (Game|Player|GetPlayerPawn 0)))
  (Variables|Default|SetBP_VRCharacter_Ref _asbp_vrcharacter)
  (Class|ActorComponent|SetTickablewhenPaused (Variables|Default|GetWidget) true))

(event EventTick
  (params (DeltaSeconds :type Float%20%28single-precision%29))
  (bind _widget (Variables|Default|GetWidget))
  (Transformation|SetWorldRotation _widget (Math|Rotator|FindLookatRotation (Transformation|GetWorldLocation _widget) (Transformation|GetWorldLocation (Variables|/Game/VR_SaberRhythmGame/Blueprints/BP_VRCharacter.BP_VRCharacter_C|GetPlayerCamera (Variables|Default|GetBP_VRCharacter_Ref)))) false false))

(fn ConstructionScript)