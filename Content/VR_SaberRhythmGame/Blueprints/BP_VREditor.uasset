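; BP_VREditor is the in-VR level editor for the saber rhythm game, laying out a timeline of editable modules for the current song.
; On BeginPlay it flags the VR character as in editor mode and spawns half-beat VREditor_Module child actors from song duration and BPM, numbering whole beats.
; Stepping slides every module, opens whichever overlaps the Cube and toggles visibility at the window edges.
; Test start/stop toggles editor visibility and current-module collision.
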(event Custom|StepForward
  (bind _childactors (Actor|GetAllChildActors false))
  (bind _currentarraynumber (Variables|Default|GetCurrentArrayNumber))
  (bind _vreditor_module_ref (Variables|Default|GetVREditor%20Module%20Ref))
  (bind _returnvalue (+ _currentarraynumber 38))
  (bind _output (Utilities|Array|Get(acopy) _childactors _returnvalue))
  (if (not (Variables|Rendering|GetbHidden))
    (bind _number (CallFunction|GetNumberOfBeats))
    (if (not (>= (Variables|Default|GetCurrentArrayNumber) (* _number 2)))
      (Rendering|SetActorHiddenInGame _vreditor_module_ref true)
      (Default|DisableCollision _vreditor_module_ref)
      (Transformation|AddActorWorldOffset _childactors (Math|Vector|MakeVector 5e+01 0.0 0.0))
      (CallFunction|SetCurrentModule)
      (if (Utilities|IsValid _output)
        (Rendering|SetActorHiddenInGame _output false)))))

(event Custom|StepBackward
  (bind _childactors (Actor|GetAllChildActors false))
  (bind _currentarraynumber (Variables|Default|GetCurrentArrayNumber))
  (bind _returnvalue (+ _currentarraynumber 39))
  (bind _output (Utilities|Array|Get(acopy) _childactors _returnvalue))
  (if (not (Variables|Rendering|GetbHidden))
    (if (not (== (Variables|Default|GetCurrentArrayNumber) 0))
      (Default|DisableCollision (Variables|Default|GetVREditor%20Module%20Ref))
      (Transformation|AddActorWorldOffset _childactors (Math|Vector|MakeVector -5e+01 0.0 0.0))
      (CallFunction|SetCurrentModule)
      (if (Utilities|IsValid _output)
        (Rendering|SetActorHiddenInGame _output true)))))

(event Custom|SetCurrentModule
  (bind _asvreditor_module (Utilities|Casting|CastToVREditor_Module (Variables|/Script/Engine.ChildActorComponent|GetChildActor (Class|Actor|GetParentComponent (Utilities|Array|Get(acopy) (Collision|GetOverlappingActors (Variables|Default|GetCube) "/Game/VR_SaberRhythmGame/Blueprints/VREditor_Module.VREditor_Module_C" :!class /Script/Engine.PrimitiveComponent))))))
  (Default|CloseModule (Variables|Default|GetVREditor%20Module%20Ref))
  (bind _output_get (Variables|Default|SetVREditor%20Module%20Ref _asvreditor_module))
  (Variables|Default|SetCurrentArrayNumber (Variables|/Game/VR_SaberRhythmGame/Blueprints/VREditor_Module.VREditor_Module_C|GetArrayNumber _output_get))
  (Default|OpenModule (Variables|Default|GetVREditor%20Module%20Ref))
  (Default|EnableCollision (Variables|Default|GetVREditor%20Module%20Ref))
  (Rendering|SetActorHiddenInGame (Utilities|Array|Get(acopy) (Actor|GetAllChildActors false) (Variables|Default|GetCurrentArrayNumber)) false))

(event Custom|GenerateModules
  (bind _number (CallFunction|GetNumberOfBeats))
  (for _index (range 0 (* _number 2))
    (bind _returnvalue (AddComponent|AddChildActorComponent false (Math|Transform|MakeTransform (Math|Vector|MakeVector (* _index (Variables|Default|GetStepWidth)) 0.0 0.0) "0, 0, 0" (Variables|Default|GetScale_3D))))
    (bind _asvreditor_module (Utilities|Casting|CastToVREditor_Module (Variables|/Script/Engine.ChildActorComponent|GetChildActor _returnvalue)))
    (bind _output_get (Variables|/Game/VR_SaberRhythmGame/Blueprints/VREditor_Module.VREditor_Module_C|SetArrayNumber _asvreditor_module _index))
    (for _index_2 (range 0 _number)
      (if (== (Math|Integer|%(Integer) _output_get 2) 0)
        (Rendering|Components|TextRender|SetText (Variables|/Game/VR_SaberRhythmGame/Blueprints/VREditor_Module.VREditor_Module_C|GetTextRender _asvreditor_module) (Utilities|Text|ToText(Integer) (+ (/ _output_get 2) 1)))
        ;[1 1 1] SetupFirstModule
        (Utilities|FlowControl|DoOnce false
          (:Completed
            (if (== _index_2 0)
              (bind _output_get_2 (Variables|Default|SetVREditor%20Module%20Ref _asvreditor_module))
              (Default|OpenModule _output_get_2)
              (Default|EnableCollision _output_get_2))))))))

(event Custom|StartTest
  (bind _asvreditor_module (Utilities|Casting|CastToVREditor_Module (Utilities|Array|Get(acopy) (Actor|GetAllChildActors false) (Variables|Default|GetCurrentArrayNumber))))
  (Default|DisableCollision _asvreditor_module)
  (Rendering|SetActorHiddenInGame true))

(event Custom|StopTest
  (bind _asvreditor_module (Utilities|Casting|CastToVREditor_Module (Utilities|Array|Get(acopy) (Actor|GetAllChildActors false) (Variables|Default|GetCurrentArrayNumber))))
  (Default|EnableCollision _asvreditor_module)
  (Rendering|SetActorHiddenInGame false))

(event EventBeginPlay
  (bind _asmain_game_instance (Utilities|Casting|CastToMainGameInstance (Game|GetGameInstance)))
  (bind _output_get (Variables|Default|SetMain_Game_Instance_Ref _asmain_game_instance))
  (Variables|Default|SetCurrentSongName (Variables|/Game/VR_SaberRhythmGame/Other/MainGameInstance.MainGameInstance_C|GetCurrentSongName _output_get))
  (Audio|Components|Audio|SetSound (Variables|Default|GetAudio) (Variables|/Game/VR_SaberRhythmGame/Other/MainGameInstance.MainGameInstance_C|GetCurrentSong _output_get))
  (bind _asbp_vrcharacter (Utilities|Casting|CastToBP_VRCharacter (Game|Player|GetPlayerPawn 0)))
  (bind _output_get_2 (Variables|Default|SetBP_VRCharacter_Ref _asbp_vrcharacter))
  (Variables|/Game/VR_SaberRhythmGame/Blueprints/BP_VRCharacter.BP_VRCharacter_C|SetVREditorMode _output_get_2 true)
  (CallFunction|GenerateModules))

(fn ConstructionScript)

(fn GetNumberOfBeats
  (Variables|Default|SetBPM (Math|Conversions|ToFloat(Integer) (Variables|/Game/VR_SaberRhythmGame/Other/MainGameInstance.MainGameInstance_C|GetCurrentBPM (Variables|Default|GetMain_Game_Instance_Ref))))
  (return (Math|Float|Round (/ (Variables|/Script/Engine.SoundBase|GetDuration (Variables|/Script/Engine.AudioComponent|GetSound (Variables|Default|GetAudio))) (/ 6e+01 (Variables|Default|GetBPM))))))