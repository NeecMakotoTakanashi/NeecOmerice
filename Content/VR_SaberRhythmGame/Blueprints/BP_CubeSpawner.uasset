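; Rhythm-game spawner that launches BP_Cube notes toward the VR player in time with the current song.
; Once started, its Tick runs every half beat, reading saved SongStructure to spawn up to two cubes at grid points.
; Cube speed derives from player distance, while music starts on a delayed timer, seeking to the editor's position in editor mode.
; When audio ends it clears cubes, then ends the editor test or opens the menu.
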(event Custom|StartSpawner
  (Utilities|FlowControl|Sequence
    (:then_0
      (Utilities|FlowControl|Delay (Variables|/Game/VR_SaberRhythmGame/Other/MainGameInstance.MainGameInstance_C|GetCurrentStartOffset (Variables|Default|GetMain_Game_Instance_Ref)))
      (Actor|Tick|SetActorTickEnabled true)
      (Actor|Tick|SetActorTickInterval (/ (/ 6e+01 (Variables|Default|GetBPM)) 2.0)))
    (:then_1
      (Variables|Default|SetEnable true)
      (Utilities|Time|SetTimerbyEvent (delegate Custom|StartMusic) 2.8)
      (if (Variables|/Game/VR_SaberRhythmGame/Blueprints/BP_VRCharacter.BP_VRCharacter_C|GetVREditorMode (Variables|Default|GetBP_VRCharacter_Ref))
        (Variables|Default|SetIndexCounter (- (Variables|/Game/VR_SaberRhythmGame/Blueprints/BP_VREditor.BP_VREditor_C|GetCurrentArrayNumber (Variables|Default|GetVREditor_Ref)) 1))))))

(event Custom|StopSpawner
  ;[1 1 1] Destroy Unnecessary Cubes
  (bind _outactors (Actor|GetAllActorsOfClass "/Game/VR_SaberRhythmGame/Blueprints/BP_Cube.BP_Cube_C"))
  (for _index (range -1 (Variables|Default|GetIndexCounter))
    (if (Utilities|IsValid (Utilities|Array|Get(acopy) _outactors _index))
      (Actor|DestroyActor (Utilities|Array|Get(acopy) _outactors _index))))
  (Variables|Default|SetIsPlayingSong false)
  (Variables|Default|SetEnable false)
  (Variables|Default|SetIndexCounter -1)
  (Audio|Components|Audio|Stop (Variables|Default|GetAudio))
  (Actor|Tick|SetActorTickEnabled false))

(event Custom|StartMusic
  (bind _audio (Variables|Default|GetAudio))
  (if (Variables|Default|GetEnable)
    (if (Variables|/Game/VR_SaberRhythmGame/Blueprints/BP_VRCharacter.BP_VRCharacter_C|GetVREditorMode (Variables|Default|GetBP_VRCharacter_Ref))
      (Audio|Components|Audio|Play _audio (* (Variables|/Game/VR_SaberRhythmGame/Blueprints/BP_VREditor.BP_VREditor_C|GetCurrentArrayNumber (Variables|Default|GetVREditor_Ref)) (/ (/ 6e+01 (Variables|Default|GetBPM)) 2.0)))
      (else
        (Audio|Components|Audio|Play _audio 0.0)))
    (Variables|Default|SetIsPlayingSong true)))

(event EventBeginPlay
  (bind _asmain_game_instance (Utilities|Casting|CastToMainGameInstance (Game|GetGameInstance)))
  (Variables|Default|SetMain_Game_Instance_Ref _asmain_game_instance)
  (bind _asbp_vrcharacter (Utilities|Casting|CastToBP_VRCharacter (Game|Player|GetPlayerPawn 0)))
  (Variables|Default|SetBP_VRCharacter_Ref _asbp_vrcharacter)
  (CallFunction|SpawnerPositionSetup)
  (bind _returnvalue (Game|GetCurrentLevelName true))
  (if (Utilities|Enum|Equal(Enum) _returnvalue "Song_Editor_Map")
    (bind _outactors (Actor|GetAllActorsOfClass "/Game/VR_SaberRhythmGame/Blueprints/BP_VREditor.BP_VREditor_C"))
    (Variables|Default|SetVREditor_Ref (Utilities|Array|Get(acopy) _outactors)))
  (Variables|Default|SetBPM (Math|Conversions|ToFloat(Integer) (Variables|/Game/VR_SaberRhythmGame/Other/MainGameInstance.MainGameInstance_C|GetCurrentBPM (Variables|Default|GetMain_Game_Instance_Ref))))
  (Audio|Components|Audio|SetSound (Variables|Default|GetAudio) (Variables|/Game/VR_SaberRhythmGame/Other/MainGameInstance.MainGameInstance_C|GetCurrentSong (Variables|Default|GetMain_Game_Instance_Ref))))

(event EventTick
  (params (DeltaSeconds :type Float%20%28single-precision%29))
  (if (Variables|Default|GetEnable)
    (Utilities|FlowControl|Sequence
      (:then_0
        (bind _result (Math|Integer|IncrementInt (Variables|Default|GetIndexCounter))
          (:%20%20
            ;[1 1 1] SpawnFirstCube
            (if (not (Utilities|Enum|Equal(Enum) (.orientation (.FirstCube (Utilities|Struct|Break2CubeStruct (Utilities|Array|Get(acopy) (Variables|/Game/VR_SaberRhythmGame/Other/SaveSong.SaveSong_C|GetSongStructure (Variables|/Game/VR_SaberRhythmGame/Other/MainGameInstance.MainGameInstance_C|GetSaveData (Variables|Default|GetMain_Game_Instance_Ref))) _result)))) "NewEnumerator5"))
              (CallFunction|SpawnCube (.way (.FirstCube (Utilities|Struct|Break2CubeStruct (Utilities|Array|Get(acopy) (Variables|/Game/VR_SaberRhythmGame/Other/SaveSong.SaveSong_C|GetSongStructure (Variables|/Game/VR_SaberRhythmGame/Other/MainGameInstance.MainGameInstance_C|GetSaveData (Variables|Default|GetMain_Game_Instance_Ref))) _result)))) (Variables|Default|GetCubeSize) (.orientation (.FirstCube (Utilities|Struct|Break2CubeStruct (Utilities|Array|Get(acopy) (Variables|/Game/VR_SaberRhythmGame/Other/SaveSong.SaveSong_C|GetSongStructure (Variables|/Game/VR_SaberRhythmGame/Other/MainGameInstance.MainGameInstance_C|GetSaveData (Variables|Default|GetMain_Game_Instance_Ref))) _result)))) (.way (.FirstCube (Utilities|Struct|Break2CubeStruct (Utilities|Array|Get(acopy) (Variables|/Game/VR_SaberRhythmGame/Other/SaveSong.SaveSong_C|GetSongStructure (Variables|/Game/VR_SaberRhythmGame/Other/MainGameInstance.MainGameInstance_C|GetSaveData (Variables|Default|GetMain_Game_Instance_Ref))) _result)))) (.isred? (.FirstCube (Utilities|Struct|Break2CubeStruct (Utilities|Array|Get(acopy) (Variables|/Game/VR_SaberRhythmGame/Other/SaveSong.SaveSong_C|GetSongStructure (Variables|/Game/VR_SaberRhythmGame/Other/MainGameInstance.MainGameInstance_C|GetSaveData (Variables|Default|GetMain_Game_Instance_Ref))) _result)))))
              ;[1 1 1] SpawnSecondCube
              (if (not (Utilities|Enum|Equal(Enum) (.orientation (.SecondCube (Utilities|Struct|Break2CubeStruct (Utilities|Array|Get(acopy) (Variables|/Game/VR_SaberRhythmGame/Other/SaveSong.SaveSong_C|GetSongStructure (Variables|/Game/VR_SaberRhythmGame/Other/MainGameInstance.MainGameInstance_C|GetSaveData (Variables|Default|GetMain_Game_Instance_Ref))) _result)))) "NewEnumerator5"))
                (CallFunction|SpawnCube (.way (.SecondCube (Utilities|Struct|Break2CubeStruct (Utilities|Array|Get(acopy) (Variables|/Game/VR_SaberRhythmGame/Other/SaveSong.SaveSong_C|GetSongStructure (Variables|/Game/VR_SaberRhythmGame/Other/MainGameInstance.MainGameInstance_C|GetSaveData (Variables|Default|GetMain_Game_Instance_Ref))) _result)))) (Variables|Default|GetCubeSize) (.orientation (.SecondCube (Utilities|Struct|Break2CubeStruct (Utilities|Array|Get(acopy) (Variables|/Game/VR_SaberRhythmGame/Other/SaveSong.SaveSong_C|GetSongStructure (Variables|/Game/VR_SaberRhythmGame/Other/MainGameInstance.MainGameInstance_C|GetSaveData (Variables|Default|GetMain_Game_Instance_Ref))) _result)))) (.way (.SecondCube (Utilities|Struct|Break2CubeStruct (Utilities|Array|Get(acopy) (Variables|/Game/VR_SaberRhythmGame/Other/SaveSong.SaveSong_C|GetSongStructure (Variables|/Game/VR_SaberRhythmGame/Other/MainGameInstance.MainGameInstance_C|GetSaveData (Variables|Default|GetMain_Game_Instance_Ref))) _result)))) (.isred? (.SecondCube (Utilities|Struct|Break2CubeStruct (Utilities|Array|Get(acopy) (Variables|/Game/VR_SaberRhythmGame/Other/SaveSong.SaveSong_C|GetSongStructure (Variables|/Game/VR_SaberRhythmGame/Other/MainGameInstance.MainGameInstance_C|GetSaveData (Variables|Default|GetMain_Game_Instance_Ref))) _result))))))))))
      (:then_1
        ;[1 1 1] AutoStop
        (if (Variables|Default|GetIsPlayingSong)
          (if (not (Audio|Components|Audio|IsPlaying (Variables|Default|GetAudio)))
            (CallFunction|StopSpawner)
            (bind _returnvalue (Game|GetCurrentLevelName true))
            (if (Utilities|Enum|Equal(Enum) _returnvalue "Song_Editor_Map")
              (Default|StopTest (Variables|Default|GetBP_VRCharacter_Ref))
              (else
                (Game|OpenLevel(byName) "Menu_Map")))))))))

(fn ConstructionScript)

(fn GetNumberOfBits
  (return (Math|Float|Round (/ (Variables|/Script/Engine.SoundBase|GetDuration (Variables|/Script/Engine.AudioComponent|GetSound (Variables|Default|GetAudio))) (/ 6e+01 (Variables|Default|GetBPM))))))

(fn SpawnCube
  (params (Index :type Way_v2%20Enum :default "NewEnumerator5") (CubeSize :type Float%20%28double-precision%29) (Orientation :type Orientation%20Enum :default "NewEnumerator5") (Way :type Way_v2%20Enum :default "NewEnumerator5") (isRed :type Boolean))
  (bind _topl (Variables|Default|GetTopL))
  (bind _downr (Variables|Default|GetDownR))
  (bind _downl (Variables|Default|GetDownL))
  (bind _topr (Variables|Default|GetTopR))
  (bind _middler (Variables|Default|GetMiddleR))
  (bind _middlel (Variables|Default|GetMiddleL))
  (bind _topm (Variables|Default|GetTopM))
  (bind _middlem (Variables|Default|GetMiddleM))
  (bind _downm (Variables|Default|GetDownM))
  (bind _returnvalue (Utilities|Select :Index Index :NewEnumerator5 _topr :NewEnumerator0 _topl :NewEnumerator1 _downr :NewEnumerator6 _downl :NewEnumerator7 0 :NewEnumerator8 _middler :NewEnumerator9 _middlel :NewEnumerator10 _topm :NewEnumerator11 _middlem :NewEnumerator12 _downm))
  (Game|SpawnActorfromClass "/Game/VR_SaberRhythmGame/Blueprints/BP_Cube.BP_Cube_C" (Math|Transform|MakeTransform (Transformation|GetWorldLocation _returnvalue) (Transformation|GetWorldRotation _returnvalue) (Math|Vector|MakeVector CubeSize CubeSize CubeSize)) "Undefined" 0 Orientation Way (/ (- (.x (Transformation|GetActorLocation (Variables|Default|GetBP_VRCharacter_Ref))) (.x (Transformation|GetActorLocation))) 3.0) isRed 0))

(fn SpawnerPositionSetup
  (bind _bp_vrcharacter_ref (Variables|Default|GetBP_VRCharacter_Ref))
  (bind _returnvalue (Transformation|GetActorLocation _bp_vrcharacter_ref))
  (Transformation|SetActorLocation (Math|Vector|MakeVector (- (.x _returnvalue) 2e+03) (.y _returnvalue) (- (.z _returnvalue) 2e+01)) false false))