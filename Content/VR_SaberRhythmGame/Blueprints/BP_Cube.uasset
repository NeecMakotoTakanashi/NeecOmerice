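; Note cube for a VR saber rhythm game, colored red or blue, showing a direction marker or a bomb mesh per its Orientation.
; Tick moves it through FlyVector, fed by a Timeline curve that starts on BeginPlay.
; A one-shot Kick event switches Tick to KickVector, disables collision and destroys the actor after a short delay.
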(event Custom|Kick
  (params (Orientation :type Orientation%20Enum :default "NewEnumerator5"))
  (Utilities|FlowControl|DoOnce false
    (:Completed
      (Variables|Default|SetisKick true)
      (Collision|SetActorEnableCollision false)
      (Utilities|FlowControl|Delay 0.5)
      (Actor|DestroyActor))))

(event EventBeginPlay
  (Variables|Default|SetStartPosition (Transformation|GetActorLocation))
  (bind _asbp_vrcharacter (Utilities|Casting|CastToBP_VRCharacter (Game|Player|GetPlayerPawn 0)))
  (Variables|Default|SetBP_VRCharacter_Ref _asbp_vrcharacter)
  (switch Utilities|FlowControl|Switch|SwitchonOrientation (Variables|Default|GetOrientation)
    (:NewEnumerator5
      _)
    (:NewEnumerator0
      (Rendering|SetVisibility (Variables|Default|GetDown) true false))
    (:NewEnumerator1
      (Rendering|SetVisibility (Variables|Default|GetUp) true false))
    (:NewEnumerator2
      (Rendering|SetVisibility (Variables|Default|GetRight) true false))
    (:NewEnumerator3
      (Rendering|SetVisibility (Variables|Default|GetLeft) true false))
    (:NewEnumerator7
      (Rendering|SetVisibility (Variables|Default|GetBomb) true false)
      (Rendering|SetVisibility (Variables|Default|GetCube) false false)
      (Collision|SetCollisionEnabled (Variables|Default|GetCube) "NoCollision")))
  (Rendering|Material|SetMaterial (Variables|Default|GetCube) 0 (select (Variables|Default|GetisRed) "/Game/VR_SaberRhythmGame/Materials/Red_M_Inst.Red_M_Inst" "/Game/VR_SaberRhythmGame/Materials/Blue_M_Inst.Blue_M_Inst"))
  (bind _cube_fly_vector (Timeline|Timeline_0 Play)))

(event EventTick
  (params (DeltaSeconds :type Float%20%28single-precision%29))
  (if (Variables|Default|GetisKick)
    (Transformation|SetActorLocation (|KickVector (stale Custom|Kick Orientation)) false false)
    (else
      (Transformation|SetActorLocation (|FlyVector DeltaSeconds (stale EventBeginPlay _cube_fly_vector)) false false))))

(fn ConstructionScript)