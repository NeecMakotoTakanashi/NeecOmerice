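; Work-in-progress 3D menu actor for a music game, stepping through genre, song and difficulty selection.
; Test left/right inputs move the current layer's index, while OK and Back change layers.
; Timelines slide and fade genre objects, song sheet and glasses, with dynamic materials and a parameter collection driving highlights and opacity.
; OK_Level opens a map per genre, but nothing here calls it and its song switches are empty.
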(event Custom|Genre_Select
  (bind _genre_objects_array (Variables|Default|GetGenre_Objects_Array))
  ;[1 1 1] Select_Effect＿ジャンルを選択したオブジェクトが光る
  ;;[1 1 1] 現在のジャンル数
  (bind _output_get (Variables|Default|SetGenre_MaxItem (Utilities|Array|Length (Utilities|Array|MakeArray (Variables|Default|GetGanre_01_Kawaii) (Variables|Default|GetGanre_02_Space) (Variables|Default|GetGanre_03_School) (Variables|Default|GetGanre_04_Halloween) (Variables|Default|GetGanre_05_Summer) (Variables|Default|GetGanre_06_Classroom)))))
  (Rendering|Material|SetMaterial _genre_objects_array 0 (Utilities|Array|Get(acopy) (Variables|Default|GetGenre_MI) _output_get))
  (bind _returnvalue (Rendering|Material|CreateDynamicMaterialInstance (Utilities|Array|Get(acopy) _genre_objects_array (Variables|Default|GetGenre_Numver)) 0 (Utilities|Array|Get(acopy) (Variables|Default|GetGenre_MI) _output_get) "" :!class /Script/Engine.PrimitiveComponent))
  (Rendering|Material|SetVectorParameterValue _returnvalue "Emissive_Color" "(R=1.000000,G=0.276635,B=0.000000,A=1.000000)" :!class /Script/Engine.MaterialInstanceDynamic)
  (bind _anim (Timeline|タイムライン PlayFromStart)
    (:Update
      (Rendering|Material|SetScalarParameterValue _returnvalue "Emissive" _anim :!class /Script/Engine.MaterialInstanceDynamic))))

(event Custom|Select_Difficulty
  ;[1 1 1] 難易度を選択する
  (Rendering|Material|SetMaterial (Variables|Default|GetPr_Theme00_Copita_001_Wong) 0 "/Game/Project_Omerice/01_Fix/Prop/Pr_Theme00/Pr_Theme00_Menu_Wong/Pr_Theme00_Copita_001_Wong/MI_Theme00_Copita_001_Wong.MI_Theme00_Copita_001_Wong")
  (Rendering|Material|SetMaterial (Variables|Default|GetPr_Theme00_CocktailGlass_001_Wong) 0 "/Game/Project_Omerice/01_Fix/Prop/Pr_Theme00/Pr_Theme00_Menu_Wong/Pr_Theme00_Copita_001_Wong/MI_Theme00_Copita_001_Wong.MI_Theme00_Copita_001_Wong")
  (Rendering|Material|SetMaterial (Variables|Default|GetPr_Theme00_CopitaLiquid_001_Wong) 0 "/Game/Project_Omerice/01_Fix/Prop/Pr_Theme00/Pr_Theme00_Menu_Wong/M_Liquid_001.M_Liquid_001")
  (Rendering|Material|SetMaterial (Variables|Default|GetPr_Theme00_CocktailGlassLiquid_001_Wong) 0 "/Game/Project_Omerice/01_Fix/Prop/Pr_Theme00/Pr_Theme00_Menu_Wong/M_Liquid_001.M_Liquid_001")
  (switch int (Math|Integer|Clamp(Integer) (Variables|Default|GetDifficulty_Num) 0 1)
    (:0
      (bind _returnvalue (Rendering|Material|CreateDynamicMaterialInstance (Variables|Default|GetPr_Theme00_CocktailGlassLiquid_001_Wong) 0 "/Game/Project_Omerice/01_Fix/Prop/Pr_Theme00/Pr_Theme00_Menu_Wong/M_Liquid_001.M_Liquid_001" "" :!class /Script/Engine.PrimitiveComponent))
      (Rendering|Material|SetVectorParameterValue _returnvalue "Emissive_Color" (Variables|Default|Getselect_EmissiveColor) :!class /Script/Engine.MaterialInstanceDynamic)
      (bind _anim (Timeline|タイムライン_7 PlayFromStart)
        (:Update
          (Rendering|Material|SetScalarParameterValue _returnvalue "Emissive" _anim :!class /Script/Engine.MaterialInstanceDynamic))))
    (:1
      (bind _returnvalue_2 (Rendering|Material|CreateDynamicMaterialInstance (Variables|Default|GetPr_Theme00_CopitaLiquid_001_Wong) 0 "/Game/Project_Omerice/01_Fix/Prop/Pr_Theme00/Pr_Theme00_Menu_Wong/M_Liquid_001.M_Liquid_001" "" :!class /Script/Engine.PrimitiveComponent))
      (Rendering|Material|SetVectorParameterValue _returnvalue_2 "Emissive_Color" (Variables|Default|Getselect_EmissiveColor) :!class /Script/Engine.MaterialInstanceDynamic)
      (bind _anim_2 (Timeline|タイムライン_8 PlayFromStart)
        (:Update
          (Rendering|Material|SetScalarParameterValue _returnvalue_2 "Emissive" _anim_2 :!class /Script/Engine.MaterialInstanceDynamic))))))

(event Custom|OK_Level
  (bind _genre_select_song_maxitem (Variables|Default|GetGenre_Select_Song_MaxItem))
  (bind _genre_numver (Variables|Default|GetGenre_Numver))
  (bind _returnvalue (- _genre_select_song_maxitem 1))
  (bind _returnvalue_2 (Math|Integer|Clamp(Integer) _genre_numver 0 _returnvalue))
  ;[1 1 1] ジャンル、曲に合わせたＬｅｖｅｌを探す
  (switch int (Variables|Default|Getselect_Genre_FInd)
    (:0
      ;;[1 1 1] コメント
      (switch Utilities|FlowControl|Switch|SwitchonSong_Kawaii (Utilities|Array|Get(acopy) (Utilities|Array|MakeArray "NewEnumerator0" "NewEnumerator1" "NewEnumerator2") _returnvalue_2)
        (:NewEnumerator0
          _)
        (:NewEnumerator1
          _)
        (:NewEnumerator2
          _))
      ;[1 1 1] 各レベルを読み込む
      (Game|OpenLevel(byObjectReference) "/Game/Project_Omerice/Maps/01_Cute_Map.01_Cute_Map"))
    (:1
      ;;[1 1 1] コメント
      (switch Utilities|FlowControl|Switch|SwitchonSong_Space (Utilities|Array|Get(acopy) (Utilities|Array|MakeArray "NewEnumerator0" "NewEnumerator1" "NewEnumerator2" "NewEnumerator3" "NewEnumerator4") _returnvalue_2)
        (:NewEnumerator0
          _)
        (:NewEnumerator1
          _)
        (:NewEnumerator2
          _)
        (:NewEnumerator3
          _)
        (:NewEnumerator4
          _))
      (Game|OpenLevel(byObjectReference) "/Game/Project_Omerice/Maps/02_Space_Map.02_Space_Map"))
    (:2
      ;;[1 1 1] コメント
      (switch Utilities|FlowControl|Switch|SwitchonSong_School (Utilities|Array|Get(acopy) (Utilities|Array|MakeArray "NewEnumerator0") _returnvalue_2)
        (:NewEnumerator0
          (Game|OpenLevel(byObjectReference) "/Game/Project_Omerice/Maps/03_Classroom_Map.03_Classroom_Map"))))
    (:3
      ;;[1 1 1] コメント
      (switch Utilities|FlowControl|Switch|SwitchonSong_Halloween (Utilities|Array|Get(acopy) (Utilities|Array|MakeArray "NewEnumerator0" "NewEnumerator1") _returnvalue_2)
        (:NewEnumerator0
          _)
        (:NewEnumerator1
          _))
      (Game|OpenLevel(byObjectReference) "/Game/Project_Omerice/Maps/04_Halloween_Map.04_Halloween_Map"))
    (:4
      ;;[1 1 1] コメント
      (switch Utilities|FlowControl|Switch|SwitchonSong_Summer (Utilities|Array|Get(acopy) (Utilities|Array|MakeArray "NewEnumerator0") _returnvalue_2)
        (:NewEnumerator0
          (Game|OpenLevel(byObjectReference) "/Game/Project_Omerice/Maps/05_Summer_Festival_Map.05_Summer_Festival_Map"))))
    (:5
      ;;[1 1 1] コメント
      (switch Utilities|FlowControl|Switch|SwitchonSong_Park (Utilities|Array|Get(acopy) (Utilities|Array|MakeArray "NewEnumerator0") _returnvalue_2)
        (:NewEnumerator0
          (Game|OpenLevel(byObjectReference) "/Game/Project_Omerice/Maps/06_ThemePark_Map.06_ThemePark_Map"))))))

(event Custom|ReturnGenre
  (bind _song_menu_00 (Variables|Default|GetSong_Menu_00))
  (bind _genre_numver (Variables|Default|GetGenre_Numver))
  (bind _genre_default_pos (Variables|Default|GetGenre_Default_Pos))
  (bind _ganre_01_kawaii (Variables|Default|GetGanre_01_Kawaii))
  (bind _ganre_02_space (Variables|Default|GetGanre_02_Space))
  (bind _ganre_04_halloween (Variables|Default|GetGanre_04_Halloween))
  (bind _ganre_05_summer (Variables|Default|GetGanre_05_Summer))
  (bind _ganre_06_classroom (Variables|Default|GetGanre_06_Classroom))
  (bind _ganre_03_school (Variables|Default|GetGanre_03_School))
  (bind _returnvalue (Transformation|GetWorldLocation _song_menu_00))
  (bind _output (Utilities|Array|Get(acopy) _genre_default_pos _genre_numver))
  (bind _array (Utilities|Array|MakeArray _ganre_01_kawaii _ganre_02_space _ganre_03_school _ganre_04_halloween _ganre_05_summer _ganre_06_classroom))
  (bind _output_2 (Utilities|Array|Get(acopy) _array _genre_numver))
  ;[1 1 1] ジャンル選択画面に戻る挙動
  (Utilities|FlowControl|Sequence
    (:then_0
      (bind _新規track_3 (Timeline|TL_Return PlayFromStart)
        (:Update
          (Transformation|SetWorldLocation _output_2 (Math|Vector|MakeVector (Math|Float|Lerp (.x (Transformation|GetWorldLocation _output_2)) (.x _output) _新規track_3) (.y _output) (.z _output)) false false)
          (Variables|Default|SetMath_Number (Variables|Default|GetGenreTmp)))))
    (:then_1
      ;[1 1 1] 選ばれなかったジャンルが表示される
      (Utilities|FlowControl|Delay 1.0)
      (for (_array_element _array_index) (Variables|Default|GetGenre_Objects_Array)
        (if (!= _array_index (Variables|Default|GetGenre_Numver))
          (Rendering|Material|SetMaterial _array_element 0 (Utilities|Array|Get(acopy) (Variables|Default|GetGenre_MI) (Utilities|Array|Length (Utilities|Array|MakeArray (Variables|Default|GetGanre_01_Kawaii) (Variables|Default|GetGanre_02_Space) (Variables|Default|GetGanre_03_School) (Variables|Default|GetGanre_04_Halloween) (Variables|Default|GetGanre_05_Summer) (Variables|Default|GetGanre_06_Classroom)))))
          (bind _新規track_0 (Timeline|タイムライン_9 PlayFromStart)
            (:Update
              (Rendering|Material|SetScalarParameterValue "/Game/Project_Omerice/01_Fix/Prop/Pr_Theme00/Pr_Theme00_Menu_Wong/Pr_Theme00_Coaster_001_Yasuda/MPC_Coaster_Opacity.MPC_Coaster_Opacity" "Opacity" _新規track_0 :!class /Script/Engine.KismetMaterialLibrary))))))
    (:then_2
      ;[1 1 1] のいて消えるメニュー
      (bind _新規track_0_2 (Timeline|タイムライン_15 PlayFromStart) ; 1you
        (:Update
          (Transformation|SetWorldLocation _song_menu_00 (Math|Vector|MakeVector (Math|Float|Lerp (.x _returnvalue) (.x (Transformation|GetWorldLocation (Variables|Default|GetAnim_Position_Menu1))) _新規track_0_2) (.y _returnvalue) (.z _returnvalue)) false false)
          (Rendering|Material|SetScalarParameterValueonMaterials (Variables|Default|GetSongs_Root) "Opacity" (- 1.0 _新規track_0_2)))))))

(event Custom|OK_Song
  (bind _pr_theme00_cocktailglass_001_wong (Variables|Default|GetPr_Theme00_CocktailGlass_001_Wong))
  (bind _pr_theme00_copita_001_wong (Variables|Default|GetPr_Theme00_Copita_001_Wong))
  (bind _song_difficulty_objects (Variables|Default|GetSong_Difficulty_Objects))
  (bind _song_menu_00 (Variables|Default|GetSong_Menu_00))
  (bind _returnvalue (Transformation|GetWorldLocation _song_menu_00))
  (bind _returnvalue_2 (Transformation|GetWorldLocation _pr_theme00_cocktailglass_001_wong))
  (bind _returnvalue_3 (Transformation|GetWorldLocation _pr_theme00_copita_001_wong))
  ;[1 1 1] メニューが退いて
  (bind _新規track_0 (Timeline|タイムライン_6 PlayFromStart)
    (:Update
      (Utilities|FlowControl|Sequence
        (:then_0
          (Transformation|SetWorldLocation _song_menu_00 (Math|Vector|MakeVector (Math|Float|Lerp (.x _returnvalue) (.x (Transformation|GetWorldLocation (Variables|Default|GetAnim_Position_Menu1))) _新規track_0) (.y _returnvalue) (.z _returnvalue)) false false)
          (Rendering|Material|SetScalarParameterValueonMaterials (Variables|Default|GetSongs_Root) "Opacity" (- 1.0 _新規track_0))
          (Rendering|Material|SetScalarParameterValueonMaterials (Variables|Default|GetSongs_Array) "Opacity" (- 1.0 _新規track_0)))
        (:then_1
          (Development|SetHiddeninGame _song_difficulty_objects false true)
          (Rendering|Material|SetScalarParameterValueonMaterials _song_difficulty_objects "Opacity" (* _新規track_0 0.5)))
        (:then_2
          ;[1 1 1] 難易度かんたんのグラスが前に出てくる
          (bind _新規track_0_2 (Timeline|タイムライン_3 PlayFromStart) ; 1you
            (:Update
              (Transformation|SetWorldLocation (Variables|Default|GetSong_Difficulty_Easy) (Math|Vector|MakeVector (Math|Float|Lerp (.x _returnvalue_2) (.x (Transformation|GetWorldLocation (Variables|Default|GetAnim_Position_Difficulty))) _新規track_0_2) (.y _returnvalue_2) (.z _returnvalue_2)) false false))))
        (:then_3
          ;[1 1 1] 難易度難しいのグラスが前に出てくる
          (Utilities|FlowControl|Delay 0.1)
          (bind _新規track_0_3 (Timeline|タイムライン_5 PlayFromStart) ; 1you
            (:Update
              (Transformation|SetWorldLocation (Variables|Default|GetSong_Difficulty_Hard) (Math|Vector|MakeVector (Math|Float|Lerp (.x _returnvalue_3) (.x (Transformation|GetWorldLocation (Variables|Default|GetAnim_Position_Difficulty))) _新規track_0_3) (.y _returnvalue_3) (.z _returnvalue_3)) false false))))))))

(event Custom|Song_select
  (bind _genre_in_songs (Variables|Default|GetGenre_in_Songs))
  (bind _select_genre_find (Variables|Default|Getselect_Genre_FInd))
  (bind _output (Utilities|Array|Get(acopy) _genre_in_songs _select_genre_find))
  ;[1 1 1] ジャンル内の曲数Ｍａｘを超えた数字の時は、Ｍａｘの数値にとどまるよう表示する
  (CallFunction|SongNameSelectDebugColor _output)
  (Variables|Default|SetGenre_Select_Song_MaxItem _output))

(event Custom|ReturnSong
  ;[1 1 1] 曲選択画面に戻る
  (bind _新規track_0 (Timeline|タイムライン_10 PlayFromStart) ; 1you
    (:Update
      (for (_array_element _array_index) (Variables|Default|GetGlasses_Root)
        (Transformation|SetWorldLocation _array_element (Math|Vector|MakeVector (Math|Float|Lerp (.X (Math|Vector|BreakVector (Transformation|GetWorldLocation _array_element))) (.X (Math|Vector|BreakVector (Utilities|Array|Get(acopy) (Variables|Default|GetDifficulty_Default_Pos) _array_index))) _新規track_0) (.Y (Math|Vector|BreakVector (Transformation|GetWorldLocation _array_element))) (.Z (Math|Vector|BreakVector (Transformation|GetWorldLocation _array_element)))) false false)
        (Rendering|Material|SetScalarParameterValueonMaterials (Variables|Default|GetSong_Difficulty_Objects) "Opacity" (* (- 1.0 _新規track_0) 0.5))
        (Rendering|Material|SetScalarParameterValueonMaterials (Variables|Default|GetSongs_Root) "Opacity" _新規track_0)
        (Rendering|Material|SetScalarParameterValueonMaterials (Variables|Default|GetSongs_Array) "Opacity" _新規track_0)
        (CallFunction|GenreinSongsNumber (Variables|Default|Getselect_Genre_FInd))
        (Variables|Default|SetMath_Number (Variables|Default|GetSongTmp))))
    (:Finished
      (Development|SetHiddeninGame (Variables|Default|GetGlasses_Root) true true))))

(event Custom|Genre_OK
  (bind _genre_numver (Variables|Default|GetGenre_Numver))
  (bind _ganre_01_kawaii (Variables|Default|GetGanre_01_Kawaii))
  (bind _ganre_02_space (Variables|Default|GetGanre_02_Space))
  (bind _ganre_04_halloween (Variables|Default|GetGanre_04_Halloween))
  (bind _ganre_05_summer (Variables|Default|GetGanre_05_Summer))
  (bind _ganre_06_classroom (Variables|Default|GetGanre_06_Classroom))
  (bind _ganre_03_school (Variables|Default|GetGanre_03_School))
  (bind _ganre_01_kawaii_2 (Variables|Default|GetGanre_01_Kawaii))
  (bind _ganre_02_space_2 (Variables|Default|GetGanre_02_Space))
  (bind _ganre_04_halloween_2 (Variables|Default|GetGanre_04_Halloween))
  (bind _ganre_05_summer_2 (Variables|Default|GetGanre_05_Summer))
  (bind _ganre_06_classroom_2 (Variables|Default|GetGanre_06_Classroom))
  (bind _ganre_03_school_2 (Variables|Default|GetGanre_03_School))
  (bind _array (Utilities|Array|MakeArray _ganre_01_kawaii _ganre_02_space _ganre_03_school _ganre_04_halloween _ganre_05_summer _ganre_06_classroom))
  (bind _array_2 (Utilities|Array|MakeArray _ganre_01_kawaii_2 _ganre_02_space_2 _ganre_03_school_2 _ganre_04_halloween_2 _ganre_05_summer_2 _ganre_06_classroom_2))
  (bind _returnvalue (Utilities|Array|Length _array_2))
  (bind _output (Utilities|Array|Get(acopy) _array _genre_numver))
  (bind _returnvalue_2 (Transformation|GetWorldLocation _output))
  ;[1 1 1] 選択したジャンルのオブジェクトがアニメーションし、選ばなかったほかのジャンルオブジェクトは非表示になる
  ;;[1 1 1] 選択したジャンル以外は
  (for (_array_element _array_index) (Variables|Default|GetGenre_Objects_Array)
    (if (!= _array_index (Variables|Default|GetGenre_Numver))
      (Variables|Default|SetGenre_MaxItem _returnvalue)
      ;;[1 1 1] 0.5秒で消える
      (Rendering|Material|SetMaterial _array_element 0 (Utilities|Array|Get(acopy) (Variables|Default|GetGenre_MI) _returnvalue))
      (bind _新規track_0 (Timeline|タイムライン_1 PlayFromStart)
        (:Update
          (Rendering|Material|SetScalarParameterValue "/Game/Project_Omerice/01_Fix/Prop/Pr_Theme00/Pr_Theme00_Menu_Wong/Pr_Theme00_Coaster_001_Yasuda/MPC_Coaster_Opacity.MPC_Coaster_Opacity" "Opacity" _新規track_0 :!class /Script/Engine.KismetMaterialLibrary)
          (Utilities|FlowControl|Delay 0.4)
          ;[1 1 1] メニューオブジェクトの表示
          (CallFunction|SongMenus)
          ;[1 1 1] Genre_Object_Anim
          (bind _新規track_0_2 (Timeline|タイムライン_0 PlayFromStart)
            (:Update
              (Transformation|SetWorldLocation _output (Math|Vector|MakeVector (Math|Float|Lerp (.x (Transformation|GetWorldLocation (Variables|Default|GetAnim_Position_Genre))) (.x _returnvalue_2) _新規track_0_2) (.y _returnvalue_2) (.z _returnvalue_2)) false false))))))))

(event Custom|Song_Menus
  (bind _song_menu_00 (Variables|Default|GetSong_Menu_00))
  (bind _genretmp (Variables|Default|GetGenreTmp))
  (bind _m_menupaper_00 (Variables|Default|GetM_MenuPaper_00))
  (bind _returnvalue (Transformation|GetWorldLocation _song_menu_00))
  (bind _output (Utilities|Array|Get(acopy) _m_menupaper_00 _genretmp))
  ;[1 1 1] 「ジャンル」を選ぶと、ジャンルに合わせた、「メニュー」オブジェクト（Texture変更による見た目の差異）が表示される
  (Utilities|FlowControl|Sequence
    (:then_0
      ;;[1 1 1] Menuモデル表示_識別テスト
      (Rendering|Material|SetMaterial (Variables|Default|GetSongs_Root) 0 _output)
      (Variables|Default|Setselect_Genre _output)
      (bind _output_get (Variables|Default|Setselect_Genre_FInd (Utilities|Array|FindItem _m_menupaper_00 (Variables|Default|Getselect_Genre))))
      (switch int _output_get
        (:0
          ;;[1 1 1] ジャンルごとの曲数に合わせた表示
          (CallFunction|SongNameGenresMaxItem (Variables|Default|GetSongs_Cute)))
        (:1
          (CallFunction|SongNameGenresMaxItem (Variables|Default|GetSongs_Space)))
        (:2
          (CallFunction|SongNameGenresMaxItem (Variables|Default|GetSongs_Classroom)))
        (:3
          (CallFunction|SongNameGenresMaxItem (Variables|Default|GetSongs_Halloween)))
        (:4
          (CallFunction|SongNameGenresMaxItem (Variables|Default|GetSongs_SummerFestival)))
        (:5
          (CallFunction|SongNameGenresMaxItem (Variables|Default|GetSongs_ThemePark))))
      (CallFunction|SongSelect))
    (:then_1
      (bind _新規track_0 (Timeline|タイムライン_12 PlayFromStart) ; 1you
        (:Update
          (Transformation|SetWorldLocation _song_menu_00 (Math|Vector|MakeVector (Math|Float|Lerp (.x _returnvalue) (.x (Transformation|GetWorldLocation (Variables|Default|GetAnim_Position_Difficulty))) _新規track_0) (.y _returnvalue) (.z _returnvalue)) false false)
          (Rendering|Material|SetScalarParameterValueonMaterials (Variables|Default|GetSongs_Root) "Opacity" _新規track_0))))))

(event EventBeginPlay
  (bind _song_name_00 (Variables|Default|GetSong_Name_00))
  (bind _pr_theme00_cocktailglass_001_wong (Variables|Default|GetPr_Theme00_CocktailGlass_001_Wong))
  (bind _pr_theme00_copita_001_wong (Variables|Default|GetPr_Theme00_Copita_001_Wong))
  (bind _ganre_01_kawaii (Variables|Default|GetGanre_01_Kawaii))
  (bind _ganre_02_space (Variables|Default|GetGanre_02_Space))
  (bind _ganre_04_halloween (Variables|Default|GetGanre_04_Halloween))
  (bind _ganre_05_summer (Variables|Default|GetGanre_05_Summer))
  (bind _ganre_06_classroom (Variables|Default|GetGanre_06_Classroom))
  (bind _ganre_03_school (Variables|Default|GetGanre_03_School))
  (bind _song_name_04 (Variables|Default|GetSong_Name_04))
  (bind _song_name_03 (Variables|Default|GetSong_Name_03))
  (bind _song_name_02 (Variables|Default|GetSong_Name_02))
  (bind _song_name_01 (Variables|Default|GetSong_Name_01))
  (bind _array (Utilities|Array|MakeArray _ganre_01_kawaii _ganre_02_space _ganre_03_school _ganre_04_halloween _ganre_05_summer _ganre_06_classroom))
  (bind _array_2 (Utilities|Array|MakeArray _song_name_00 _song_name_01 _song_name_02 _song_name_03 _song_name_04))
  ;[1 1 1] 初期設定
  (Utilities|FlowControl|Sequence
    (:then_0
      (Input|EnableInput (Game|GetPlayerController 0))
      (Variables|Default|SetIn_OK false)
      (Variables|Default|SetLayerCount 0)
      ;[1 1 1] 現在のジャンル数
      (Variables|Default|SetGenre_MaxItem (Utilities|Array|Length _array))
      ;[1 1 1] 全オブジェクト呼び出し
      (Variables|Default|SetGenre_Objects_Array _array)
      ;[1 1 1] オブジェクト指定
      (Variables|Default|SetSelect_Genre_Object (Utilities|Array|Get(acopy) _array))
      (Variables|Default|SetGenre_Default_Pos (Utilities|Array|MakeArray (Transformation|GetWorldLocation _ganre_01_kawaii) (Transformation|GetWorldLocation _ganre_02_space) (Transformation|GetWorldLocation _ganre_03_school) (Transformation|GetWorldLocation _ganre_04_halloween) (Transformation|GetWorldLocation _ganre_05_summer) (Transformation|GetWorldLocation _ganre_06_classroom)))
      ;[1 1 1] 曲選択画面全オブジェクト
      (bind _output_get (Variables|Default|SetSongs_Root (Utilities|Array|MakeArray (Variables|Default|GetSong_Menu_00) _song_name_00 _song_name_01 _song_name_02 _song_name_03 _song_name_04)))
      (Rendering|Material|SetScalarParameterValueonMaterials _output_get "Opacity" 0.0)
      ;[1 1 1] 全曲
      (Variables|Default|SetSongs_Array _array_2)
      ;[1 1 1] 曲を選ぶ
      (Variables|Default|Setselect_Song_Name (Utilities|Array|Get(acopy) _array_2 (Variables|Default|GetGenre_Numver)))
      ;[1 1 1] 全曲数
      (Variables|Default|SetSong_MaxItem (Utilities|Array|Length _array_2))
      ;[1 1 1] 各ジャンルの曲数
      (Variables|Default|SetSongs_Cute (|GetNumEnumEntries))
      (Variables|Default|SetSongs_Space (|GetNumEnumEntries))
      (Variables|Default|SetSongs_Classroom (|GetNumEnumEntries))
      (Variables|Default|SetSongs_Halloween (|GetNumEnumEntries))
      (Variables|Default|SetSongs_SummerFestival (|GetNumEnumEntries))
      (Variables|Default|SetSongs_ThemePark (|GetNumEnumEntries))
      ;[1 1 1] 各ジャンルの総曲数
      (Variables|Default|SetGenre_in_Songs (Utilities|Array|MakeArray (Variables|Default|GetSongs_Cute) (Variables|Default|GetSongs_Space) (Variables|Default|GetSongs_Classroom) (Variables|Default|GetSongs_Halloween) (Variables|Default|GetSongs_SummerFestival) (Variables|Default|GetSongs_ThemePark)))
      ;[1 1 1] コメント
      (Variables|Default|SetSelect_Genre_in_Songs (Utilities|Array|Get(acopy) (Utilities|Array|MakeArray (Variables|Default|GetSongs_Cute) (Variables|Default|GetSongs_Space) (Variables|Default|GetSongs_Classroom) (Variables|Default|GetSongs_Halloween) (Variables|Default|GetSongs_SummerFestival) (Variables|Default|GetSongs_ThemePark)) (Variables|Default|GetGenre_Numver)))
      ;[1 1 1] Textオブジェクト
      (bind _output_get_2 (Variables|Default|SetTRC_Song_Text (Utilities|Array|MakeArray 0 0 0 0 0)))
      ;[1 1 1] 難易度グラスの格納
      (Variables|Default|SetSong_Difficulty_Hard (Variables|Default|GetPr_Theme00_Copita_001_Wong))
      (Variables|Default|SetSong_Difficulty_Easy (Variables|Default|GetPr_Theme00_CocktailGlass_001_Wong))
      (bind _output_get_3 (Variables|Default|SetSong_Difficulty_Objects (Utilities|Array|MakeArray _pr_theme00_cocktailglass_001_wong (Variables|Default|GetPr_Theme00_CocktailGlassLiquid_001_Wong) _pr_theme00_copita_001_wong (Variables|Default|GetPr_Theme00_CopitaLiquid_001_Wong))))
      (Variables|Default|SetGlasses_Root (Utilities|Array|MakeArray _pr_theme00_cocktailglass_001_wong _pr_theme00_copita_001_wong))
      (Variables|Default|SetDifficulty_Default_Pos (Utilities|Array|MakeArray (Transformation|GetWorldLocation _pr_theme00_cocktailglass_001_wong) (Transformation|GetWorldLocation _pr_theme00_copita_001_wong)))
      (Rendering|Material|SetScalarParameterValueonMaterials _output_get_3 "Opacity" 0.0)
      (Development|SetHiddeninGame _output_get_3 true true))
    (:then_1
      (if (Variables|Default|GetIn_Controller)
        _))))

(event Collision|EventActorBeginOverlap
  (params (OtherActor :type Actor%20Object%20Reference)))

(event EventTick
  (params (DeltaSeconds :type Float%20%28single-precision%29)))

(event Input|ActionEvents|InputActionTest_OK
  (params (Key :type Key%20Structure :default "None"))
  (bind _genre_numver (Variables|Default|GetGenre_Numver))
  (bind _songnum (Variables|Default|GetSongNum))
  ;[1 1 1] OK
  (:Pressed
    (switch int (Variables|Default|GetLayerCount)
      (:Default
        _)
      (:0
        _)
      (:1
        _))
    (Variables|Default|SetLayerCount (Math|Integer|Clamp(Integer) (+ (Variables|Default|GetLayerCount) 1) 0 2))
    (switch int (Variables|Default|GetLayerCount)
      (:1
        (CallFunction|GenreOK)
        (Variables|Default|SetGenreTmp _genre_numver)
        (Development|PrintString (Utilities|String|ToString(Integer) _genre_numver) true true "(R=1.000000,G=0.523053,B=0.000000,A=1.000000)"))
      (:2
        (CallFunction|OKSong)
        (Variables|Default|SetSongTmp _songnum)
        (Development|PrintString (Utilities|String|ToString(Integer) _songnum) true true "(R=1.000000,G=0.987099,B=0.000000,A=1.000000)")))))

(event Input|ActionEvents|InputActionTest_Back
  (params (Key :type Key%20Structure :default "None"))
  ;[1 1 1] Back
  (:Pressed
    (switch int (Variables|Default|GetLayerCount)
      (:Default
        _)
      (:1
        _)
      (:2
        _))
    (Variables|Default|SetLayerCount (Math|Integer|Clamp(Integer) (- (Variables|Default|GetLayerCount) 1) 0 2))
    (switch int (Variables|Default|GetLayerCount)
      (:0
        (CallFunction|ReturnGenre))
      (:1
        (CallFunction|ReturnSong)
        (CallFunction|SongMenus)))))

(event Input|ActionEvents|InputActionTest_Right
  (params (Key :type Key%20Structure :default "None"))
  ;[1 1 1] ボタン入力
  (:Pressed
    (bind _result (Math|Integer|IncrementInt (Variables|Default|GetMath_Number))
      (:%20%20
        (Variables|Default|SetMath_Number (Math|Integer|Clamp(Integer) _result 0 (- (Variables|Default|GetGenre_MaxItem) 1)))
        (switch int (Variables|Default|GetLayerCount)
          (:0
            (Variables|Default|SetGenre_Numver (Variables|Default|GetMath_Number))
            (CallFunction|GenreSelect))
          (:1
            (Variables|Default|SetSongNum (Variables|Default|GetMath_Number))
            (CallFunction|SongSelect))
          (:2
            (Variables|Default|SetDifficulty_Num (Variables|Default|GetMath_Number))
            (CallFunction|SelectDifficulty)))))))

(event Input|ActionEvents|InputActionTest_Left
  (params (Key :type Key%20Structure :default "None"))
  ;[1 1 1] ボタン入力
  (:Pressed
    (bind _result (Math|Integer|DecrementInt (Variables|Default|GetMath_Number))
      (:%20%20
        (Variables|Default|SetMath_Number (Math|Integer|Clamp(Integer) _result 0 (- (Variables|Default|GetGenre_MaxItem) 1)))
        (switch int (Variables|Default|GetLayerCount)
          (:0
            (Variables|Default|SetGenre_Numver (Variables|Default|GetMath_Number))
            (CallFunction|GenreSelect))
          (:1
            (Variables|Default|SetSongNum (Variables|Default|GetMath_Number))
            (CallFunction|SongSelect))
          (:2
            (Variables|Default|SetDifficulty_Num (Variables|Default|GetMath_Number))
            (CallFunction|SelectDifficulty)))))))

(fn ConstructionScript
  (Development|SetHiddeninGame (Variables|Default|GetAnim_Position_Genre) (Variables|Default|GetHIdden_In_Games) false))

(fn SongSelectDebugColor
  (params (Songs_etc :type Integer))
  (bind _songs_array (Variables|Default|GetSongs_Array))
  (Rendering|Material|SetMaterial _songs_array 0 0)
  (bind _returnvalue (Rendering|Material|CreateDynamicMaterialInstance (Utilities|Array|Get(acopy) _songs_array (Math|Integer|Clamp(Integer) (Variables|Default|GetGenre_Numver) 0 (- Songs_etc 1))) 0 0 "" :!class /Script/Engine.PrimitiveComponent))
  (Rendering|Material|SetVectorParameterValue _returnvalue "TestColor" "(R=0.000000,G=0.839838,B=1.000000,A=1.000000)" :!class /Script/Engine.MaterialInstanceDynamic)
  (return))

(fn SongNameGenresMaxItem
  (params (FirstIndex :type Integer))
  (for _index (range FirstIndex (Variables|Default|GetSong_MaxItem))
    _))

(fn SongNameSelectDebugColor
  (params (NewParam :type Integer))
  (bind _song_material (Variables|Default|GetSong_Material))
  (bind _songs_array (Variables|Default|GetSongs_Array))
  (Rendering|Material|SetMaterial _songs_array 0 _song_material)
  (bind _returnvalue (Rendering|Material|CreateDynamicMaterialInstance (Utilities|Array|Get(acopy) _songs_array (Math|Integer|Clamp(Integer) (Variables|Default|GetSongNum) 0 (- NewParam 1))) 0 _song_material "" :!class /Script/Engine.PrimitiveComponent))
  (Rendering|Material|SetVectorParameterValue _returnvalue "TestColor" "(R=0.000000,G=0.839838,B=1.000000,A=1.000000)" :!class /Script/Engine.MaterialInstanceDynamic))

(fn GenreinSongsNumber
  (params (SelectGenre :type Integer))
  (switch int SelectGenre
    (:0
      (CallFunction|SongNameGenresMaxItem (Variables|Default|GetSongs_Cute)))
    (:1
      (CallFunction|SongNameGenresMaxItem (Variables|Default|GetSongs_Space)))
    (:2
      (CallFunction|SongNameGenresMaxItem (Variables|Default|GetSongs_Classroom)))
    (:3
      (CallFunction|SongNameGenresMaxItem (Variables|Default|GetSongs_Halloween)))
    (:4
      (CallFunction|SongNameGenresMaxItem (Variables|Default|GetSongs_SummerFestival)))
    (:5
      (CallFunction|SongNameGenresMaxItem (Variables|Default|GetSongs_ThemePark))))
  (return 0))